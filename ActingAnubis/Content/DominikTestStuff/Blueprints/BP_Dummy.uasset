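; BP_Dummy is a test target actor that fires spawned objects and can be destroyed through its weak spot.
; From BeginPlay, StartShooting runs on a looping one-second timer that it re-sets on each call, spawning ClassToSpawn at the ShootPoint's location and rotation.
; An actor tagged "Pullable" overlapping the WeakSpot component destroys the dummy.
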(event `self.ReceiveBeginPlay`
  (`self.Start shooting`))

(event `Start shooting`
  (bind _shootpoint (`self.ShootPoint`))
  (`KismetSystemLibrary.K2_SetTimerDelegate` (delegate `Start shooting`) 1.0 true)
  (`|SpawnActorFromClass` (`self.ClassToSpawn`) (`KismetMathLibrary.MakeTransform` (`SceneComponent.K2_GetComponentLocation` _shootpoint) (`SceneComponent.K2_GetComponentRotation` _shootpoint)) "Undefined" "MultiplyWithRoot" null null))

(event `self.WeakSpot.OnComponentBeginOverlap`
  (params (OverlappedComponent :type "PrimitiveComponent Object Reference") (OtherActor :type "Actor Object Reference") (OtherComp :type "PrimitiveComponent Object Reference") (OtherBodyIndex :type Integer) (bFromSweep :type Boolean) (SweepResult :type "HitResult Structure (by ref)"))
  (if (`self.ActorHasTag` OtherActor "Pullable")
    (`self.K2_DestroyActor`)))

(fn `UserConstructionScript`)