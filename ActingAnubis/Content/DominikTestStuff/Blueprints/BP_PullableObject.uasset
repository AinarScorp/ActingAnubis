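; BP_PullableObject is a prototype actor with a static mesh and projectile movement that serves either as a projectile or a stationary object.
; The construction script uses the IsProjectile flag to pick the mesh material and set an initial speed, zero when not a projectile.
; In projectile mode, overlapping the first-person character prints a placeholder damage message and destroys the actor.
; No pulling logic or real damage is implemented here.
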(event `self.ReceiveBeginPlay`)

(event `self.StaticMesh.OnComponentBeginOverlap`
  (params (OverlappedComponent :type "PrimitiveComponent Object Reference") (OtherActor :type "Actor Object Reference") (OtherComp :type "PrimitiveComponent Object Reference") (OtherBodyIndex :type Integer) (bFromSweep :type Boolean) (SweepResult :type "HitResult Structure (by ref)"))
  (if (`self.IsProjectile`)
    (cast `/Game/FirstPerson/Blueprints/BP_FirstPersonCharacter` OtherActor)
    (`KismetSystemLibrary.PrintString` "DAMAGE" true true (struct :`R` 1.0 :`G` 0.044076 :`A` 1.0))
    (`self.K2_DestroyActor`)))

(fn `UserConstructionScript`
  (if (`self.IsProjectile`)
    (set `ProjectileMovementComponent.InitialSpeed` 1000.0 (`self.ProjectileMovement`))
    (`PrimitiveComponent.SetMaterial` (`self.StaticMesh`) 0 "/Engine/MapTemplates/Materials/BasicAsset01.BasicAsset01")
    (else
      (set `ProjectileMovementComponent.InitialSpeed` 0.0 (`self.ProjectileMovement`))
      (`PrimitiveComponent.SetMaterial` (`self.StaticMesh`) 0 "/Engine/MapTemplates/Materials/BasicAsset03.BasicAsset03"))))