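; Dash ability component that launches the player character in a quick burst when its tagged input triggers.
; The launch follows the last movement input vector, or the actor's forward vector when there is none, scaled by DashLength and added to current velocity.
; A CanDash flag and a short Delay form the cooldown.
; It always acts on player character 0 rather than the component's owner.
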(event `Dash`
  (bind _returnvalue (`GameplayStatics.GetPlayerCharacter` 0))
  (bind _returnvalue_2 (`GameplayStatics.GetPlayerCharacter` 0))
  (bind _returnvalue_3 (`PawnMovementComponent.GetLastInputVector` (`Character.CharacterMovement` _returnvalue_2)))
  (if (`self.CanDash`)
    (set `self.CanDash` false)
    (if (== _returnvalue_3 (0.0 0.0 0.0))
      (`Character.LaunchCharacter` _returnvalue (* (`Actor.GetActorForwardVector` _returnvalue) (`self.DashLength`)) false false)
      (else
        (`Character.LaunchCharacter` _returnvalue_2 (* _returnvalue_3 (`self.DashLength`)) false false)))
    (`KismetSystemLibrary.Delay` 1.0)
    (set `self.CanDash` true)))

(event `ListenToInputTagInterface.ReceiveTriggeredInputFromTag`
  (params (EventData :type "GameplayTag Structure"))
  (`self.Dash`))

(fn `RelativeTransform`
  (returns (ReturnValue :type "Transform Structure"))
  (return))

(fn `StoreWaitAsyncTask`
  (params (WaitGameplayEvent :type "AbilityAsync_WaitGameplayEvent Object Reference"))
  (returns (ReturnValue :type Boolean))
  (return false))