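; Actor component that lets its owner pull in projectile-tagged objects, hold them in front of the camera and shoot them away.
; A pull input sphere-traces from the camera, then grabs the hit component with a found-or-created physics handle, which Tick keeps ahead of the camera.
; A shoot input releases it with an impulse along the camera's forward vector.
; A storage counter gates both actions, and gameplay events notify the object.
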(event `self.ReceiveBeginPlay`
  (set `self.PhysicsHandleComponent` (`self.GetPhysicsHandleComponent`)))

(event `self.ReceiveTick`
  (params (DeltaSeconds :type "Float (single-precision)"))
  (`/Engine/EditorBlueprintResources/StandardMacros.IsValid` (`PhysicsHandleComponent.GetGrabbedComponent` (`self.GetPhysicsHandleComponent`))
    (:`Is Valid`
      (`PhysicsHandleComponent.SetTargetLocationAndRotation` :`self` (`self.GetPhysicsHandleComponent`) :`NewLocation` (`.CameraLocationWithForwardScaled` (`/Game/_Game/Blueprints/Library/BP_GameplayUtilityLibrary.GetCameraTransformInfo` null 200.0))))))

(event `PullRaycast`
  (bind _pulledobject (`self.PulledObject`))
  (bind (_cameralocation _cameraforwardvector _camerarotation _cameralocationwithforwardscaled) (`/Game/_Game/Blueprints/Library/BP_GameplayUtilityLibrary.GetCameraTransformInfo` null (`self.PullRange`)))
  (`/Engine/EditorBlueprintResources/StandardMacros.IsValid` (`PhysicsHandleComponent.GetGrabbedComponent` (`self.GetPhysicsHandleComponent`))
    (:`Is Not Valid`
      (if (< (`self.CurrentStorage`) (`self.MaxStorage`))
        (set `self.PulledObject` null)
        (bind _outhit (`KismetSystemLibrary.SphereTraceSingle` _cameralocation _cameralocationwithforwardscaled 100.0 "TraceTypeQuery4" false (`|MakeArray` (`self.GetOwner`))))
        (bind (_bblockinghit _binitialoverlap _time _distance _location _impactpoint _normal _impactnormal _physmat _hitactor _hitcomponent) (`GameplayStatics.BreakHitResult` _outhit))
        (bind _output_get (set `self.PulledObject` _hitactor))
        (`/Engine/EditorBlueprintResources/StandardMacros.IsValid` _output_get
          (:`Is Valid`
            (bind _returnvalue (`AnubisAbilitySystemLibrary.HasAnyMatchingGameplayTags` (`self.PulledObject`) (struct :`GameplayTags` (struct :`(TagName` "Identifier.Projectile") :`(TagName` "Status.Physics.CanBePulled")))))
            (if _returnvalue
              ;[0.15 0.15 0.15 0.5 12] Same As CurrentStorage == CurrentStorage + 1
              (`/Engine/EditorBlueprintResources/StandardMacros.IncrementInt` (`self.CurrentStorage`)
                (:`  `
                  (`self.SendGameplayEvent` (struct :`TagName` "Gameplay.Event.Pull.Executed"))
                  (`PhysicsHandleComponent.GrabComponentAtLocationWithRotation` (`self.GetPhysicsHandleComponent`) _hitcomponent "None" (`Actor.K2_GetActorLocation` _pulledobject) (`Actor.K2_GetActorRotation` _pulledobject)))))))))))

(event `ListenToInputTagInterface.ReceiveTriggeredInputFromTag`
  (params (EventData :type "GameplayTag Structure"))
  (`|SwitchGameplayTag` EventData
    (:`Input.Pull.Tap`
      (`self.PullRaycast`))
    (:`Input.Shoot`
      (`self.Push`))))

(event `Push`
  (if (and (> (`self.CurrentStorage`) 0) (`KismetSystemLibrary.IsValid` (`self.PulledObject`)))
    (`/Engine/EditorBlueprintResources/StandardMacros.DecrementInt` (`self.CurrentStorage`)
      (:`  `
        (`self.ShootAndRelease`)
        (`self.ExecuteShoot`)
        (set `self.PulledObject` null)))))

(fn `ExecuteShoot`
  (`AbilitySystemBlueprintLibrary.SendGameplayEventToActor` (`self.PulledObject`) (struct :`TagName` "Gameplay.Event.Pull.Shoot") (make `GameplayEventData` :`Instigator` (`GameplayStatics.GetPlayerCharacter` 0) :`Target` (`self.PulledObject`))))

(fn `GetPhysicsHandleComponent`
  (returns (ReturnValue :type "PhysicsHandleComponent Object Reference"))
  (locals (OutPhysicsHandle :type "PhysicsHandleComponent Object Reference"))
  (`|ExecutionSequence`
    (:`then_0`
      (`self.PhysicsHandleComponent`
        (:`then`
          (return (`self.PhysicsHandleComponent`)))
        (:`else`
          (bind _output_get (set `local.OutPhysicsHandle` (`Actor.GetComponentByClass` (`self.GetOwner`) "/Script/Engine.PhysicsHandleComponent")))
          (`/Engine/EditorBlueprintResources/StandardMacros.IsValid` _output_get
            (:`Is Not Valid`
              (bind _returnvalue (`|AddComponentByClass` (`self.GetOwner`) "/Script/Engine.PhysicsHandleComponent"))
              (set `local.OutPhysicsHandle` _returnvalue))))))
    (:`then_1`
      (return (`local.OutPhysicsHandle`)))))

(fn `RelativeTransform`
  (returns (ReturnValue :type "Transform Structure"))
  (return))

(fn `SendGameplayEvent`
  (params (EventTag :type "GameplayTag Structure"))
  (bind _pulledobject (`self.PulledObject`)
    (:`then`
      (`AbilitySystemBlueprintLibrary.SendGameplayEventToActor` _pulledobject EventTag (make `GameplayEventData` :`Instigator` (`self.GetOwner`) :`Target` (`self.PulledObject`))))
    (:`else`)))

(fn `ShootAndRelease`
  (locals (PrimitiveComponent :type "PrimitiveComponent Object Reference"))
  (bind _physicshandlecomponent (`self.PhysicsHandleComponent`))
  (bind _output_get (set `local.PrimitiveComponent` (`PhysicsHandleComponent.GetGrabbedComponent` _physicshandlecomponent)))
  (`PhysicsHandleComponent.ReleaseComponent` _physicshandlecomponent)
  (`/Game/_Game/Blueprints/Library/BP_GameplayLibrary.ExecutePushOnPushableObject` (`self.PulledObject`) _output_get (`self.GetOwner`) (`/Game/_Game/Blueprints/Library/BP_GameplayUtilityLibrary.GetCameraForwardVector` null) (`self.ShootingSpeed`)))

(fn `StoreWaitAsyncTask`
  (params (WaitGameplayEvent :type "AbilityAsync_WaitGameplayEvent Object Reference"))
  (returns (ReturnValue :type Boolean))
  (return false))