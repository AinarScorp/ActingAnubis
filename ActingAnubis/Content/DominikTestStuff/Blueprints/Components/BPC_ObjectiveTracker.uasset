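; BPC_ObjectiveTracker is an objective tracker component that advances the win condition and opens the portal stage once the goal is met.
; Each UpdateProgress call increments WinConditionNum on AnubisGameMode, which holds both the count and WinGoal.
; At or above the goal it streams in the Portals level instance, with no guard against repeat loads on later calls.
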(event `UpdateProgress`
  (bind _asanubis_game_mode (cast `/Game/DominikTestStuff/Levels/Game/AnubisGameMode` (`GameplayStatics.GetGameMode`)))
  (bind _winconditionnum (`/Game/DominikTestStuff/Levels/Game/AnubisGameMode.WinConditionNum` _asanubis_game_mode))
  (set `/Game/DominikTestStuff/Levels/Game/AnubisGameMode.WinConditionNum` (+ _winconditionnum 1.0) _asanubis_game_mode)
  (if (>= _winconditionnum (`/Game/DominikTestStuff/Levels/Game/AnubisGameMode.WinGoal` _asanubis_game_mode))
    (`LevelStreamingDynamic.LoadLevelInstanceBySoftObjectPtr` "/Game/DominikTestStuff/Levels/Game/Instances/Portals.Portals" (0.0 0.0 0.0) (struct) "" null)))

(fn `RelativeTransform`
  (returns (ReturnValue :type "Transform Structure"))
  (return))

(fn `StoreWaitAsyncTask`
  (params (WaitGameplayEvent :type "AbilityAsync_WaitGameplayEvent Object Reference"))
  (returns (ReturnValue :type Boolean))
  (return false))