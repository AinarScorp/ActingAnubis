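; BP_Spikes is a spike trap hazard that damages actors entering its box, with near-lethal-scale damage for those tagged Identifier.Enemy and light damage otherwise.
; The construction script lays out a centered grid of instanced meshes from count, spacing and scale, with optional mesh and material overrides.
; TrySurroundWithCollison fits the box to the instanced mesh bounds and stores that extent, which construction reapplies.
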(event `TrySurroundWithCollison`
  (bind (_origin _boxextent) (`KismetSystemLibrary.GetComponentBounds` (`self.InstancedStaticMesh`)))
  (`BoxComponent.SetBoxExtent` (`self.Box`) _boxextent false)
  (set `self.BoxCollisionSize` _boxextent))

(event `self.Box.OnComponentBeginOverlap`
  (params (OverlappedComponent :type "PrimitiveComponent Object Reference") (OtherActor :type "Actor Object Reference") (OtherComp :type "PrimitiveComponent Object Reference") (OtherBodyIndex :type Integer) (bFromSweep :type Boolean) (SweepResult :type "HitResult Structure (by ref)"))
  (bind _returnvalue (`AnubisAbilitySystemLibrary.HasMatchingGameplayTag` OtherActor (struct :`TagName` "Identifier.Enemy")))
  (`/Game/_Game/Blueprints/Library/BP_GameplayLibrary.DealDamageToActor` OtherActor self (`KismetMathLibrary.SelectFloat` 10000.0 10.0 _returnvalue)))

(fn `UserConstructionScript`
  (locals (X :type Integer) (Y :type Integer) (StartX :type "Float (double-precision)") (StartY :type "Float (double-precision)"))
  (bind (_returnvalue_x _returnvalue_y _returnvalue_z) (`KismetMathLibrary.BreakVector` (`self.K2_GetActorLocation`)))
  (bind _spacing_betweenobjects (`self.Spacing BetweenObjects`))
  (bind (_gridamount_x _gridamount_y) (break `IntVector` (`self.GridAmount`)))
  (bind (_gridamount_x_2 _gridamount_y_2) (break `IntVector` (`self.GridAmount`)))
  (`SceneComponent.SetWorldScale3D` (`self.InstancedStaticMesh`) (1.0 1.0 1.0))
  (`InstancedStaticMeshComponent.ClearInstances` (`self.InstancedStaticMesh`))
  (`BoxComponent.SetBoxExtent` (`self.Box`) (`self.BoxCollisionSize`) false)
  (if (`KismetSystemLibrary.IsValid` (`self.OverrideMaterial`))
    (`PrimitiveComponent.SetMaterial` (`self.InstancedStaticMesh`) 0 (`self.OverrideMaterial`)))
  (if (`KismetSystemLibrary.IsValid` (`self.OverrideConemesh`))
    (`StaticMeshComponent.SetStaticMesh` (`self.InstancedStaticMesh`) (`self.OverrideConemesh`)))
  (set `local.X` (- _gridamount_x 1))
  (set `local.Y` (- _gridamount_y 1))
  (set `local.StartX` (* (* (`local.X`) 0.5 (`self.Spacing BetweenObjects`)) -1.0))
  (set `local.StartY` (* (* (`local.Y`) 0.5 (`self.Spacing BetweenObjects`)) -1.0))
  (for _index (range 1 (+ _gridamount_x_2 1))
    (set `local.X` (- _index 1))
    (for _index_2 (range 1 (+ _gridamount_y_2 1))
      (set `local.Y` (- _index_2 1))
      (`InstancedStaticMeshComponent.AddInstance` (`self.InstancedStaticMesh`) (`KismetMathLibrary.MakeTransform` (`KismetMathLibrary.MakeVector` (+ (+ (`local.StartX`) (* (`local.X`) _spacing_betweenobjects)) _returnvalue_x) (+ (+ (* _spacing_betweenobjects (`local.Y`)) (`local.StartY`)) _returnvalue_y) _returnvalue_z) (`self.K2_GetActorRotation`) (`self.MeshScale`)) true))))