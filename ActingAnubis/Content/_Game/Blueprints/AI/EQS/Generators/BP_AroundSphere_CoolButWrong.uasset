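; EQS generator that places query points on a sphere surface around each context location or actor.
; GenerateLocations derives the point count from the sphere's surface area over squared Spacing, then distributes points with a golden-ratio (Fibonacci) spiral scaled by Radius.
; Each generated point is also printed as debug output, and some unused rotation-based placement nodes remain.
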(fn `DoItemGeneration`
  (params (ContextLocations :type "Array of Vector Structure (by ref)"))
  (locals (Step :type Integer))
  (`self.GenerateLocations` ContextLocations)
  (return))

(fn `DoItemGenerationFromActors`
  (params (ContextActors :type "Array of Actor Object Reference (by ref)"))
  (locals (Locations :type "Array of Vector Structure"))
  (for _array_element ContextActors
    (`KismetArrayLibrary.Array_Add` (`local.Locations`) (`Actor.K2_GetActorLocation` _array_element)))
  (`self.GenerateLocations` (`local.Locations`))
  (return))

(fn `GenerateLocations`
  (params (Array :type "Array of Vector Structure"))
  (locals (Count :type Integer) (OriginLocation :type "Vector Structure") (SurfaceArea :type "Float (double-precision)") (phi :type "Float (double-precision)") (Mult :type "Float (double-precision)") (Add :type "Float (double-precision)") (Theta :type "Float (double-precision)") (Index :type Integer))
  (bind _phi (`local.phi`))
  (bind _theta (`local.Theta`))
  (bind _returnvalue (+ (* (`KismetMathLibrary.MakeVector` (* (`KismetMathLibrary.Sin` _phi) (`KismetMathLibrary.Cos` _theta)) (* (`KismetMathLibrary.Sin` _phi) (`KismetMathLibrary.Sin` _theta)) (`KismetMathLibrary.Cos` _phi)) (`self.Radius`)) (`local.OriginLocation`)))
  (set `local.SurfaceArea` (* (`KismetMathLibrary.GetPI`) (`KismetMathLibrary.Square` (`self.Radius`)) 4.0))
  (set `local.Count` (/ (`KismetMathLibrary.Round` (`local.SurfaceArea`)) (`KismetMathLibrary.Square` (`self.Spacing`))))
  (for _array_element Array
    (set `local.OriginLocation` _array_element)
    (for _index (range (`local.Count`))
      (bind _output_get (set `local.Index` _index))
      (bind _output_get_2 (set `local.Add` (+ _output_get 0.5)))
      (bind _output_get_3 (set `local.Mult` (* _output_get_2 2.0)))
      (set `local.phi` (`KismetMathLibrary.Acos` (- 1.0 (/ _output_get_3 (`local.Count`)))))
      (bind _output_get_4 (set `local.Add` (+ 1.0 (`KismetMathLibrary.Sqrt` 5.0))))
      (set `local.Theta` (* _output_get_4 (`KismetMathLibrary.GetPI`) (`local.Index`)))
      (`self.AddGeneratedVector` _returnvalue)
      (`KismetSystemLibrary.PrintString` (`KismetStringLibrary.Conv_VectorToString` _returnvalue)))))