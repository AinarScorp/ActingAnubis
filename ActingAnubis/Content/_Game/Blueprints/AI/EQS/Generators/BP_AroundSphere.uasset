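; BP_AroundSphere is an EQS generator that fills a sphere around each context location or actor with query points.
; It slices the sphere into horizontal disks by SpacingOnHeight, sizing each from Radius and its height offset.
; Each disk is filled with concentric rings whose point counts follow circumference over Spacing.
; A custom ProperForLoop macro provides the float-step loops, with an option to force the first iteration.
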(fn `DoItemGeneration`
  (params (ContextLocations :type "Array of Vector Structure (by ref)"))
  (locals (Step :type Integer))
  (`self.GenerateLocations` ContextLocations)
  (return))

(fn `DoItemGenerationFromActors`
  (params (ContextActors :type "Array of Actor Object Reference (by ref)"))
  (locals (Locations :type "Array of Vector Structure"))
  (for _array_element ContextActors
    (`KismetArrayLibrary.Array_Add` (`local.Locations`) (`Actor.K2_GetActorLocation` _array_element)))
  (`self.GenerateLocations` (`local.Locations`))
  (return))

(fn `GenerateLocations`
  (params (Array :type "Array of Vector Structure"))
  (locals (OriginLocation :type "Vector Structure") (DiskRadius :type "Float (double-precision)") (Z :type "Float (double-precision)") (Height :type "Float (double-precision)") (R :type "Float (double-precision)") (Circumference :type "Float (double-precision)") (PointCount :type Integer) (I :type Integer) (Angle :type "Float (double-precision)") (NumOfRings :type Integer))
  (bind (_originlocation_x _originlocation_y _originlocation_z) (`KismetMathLibrary.BreakVector` (`local.OriginLocation`)))
  (bind _radius (`self.Radius`))
  (`|ExecutionSequence`
    (:`then_1`
      (for _array_element Array
        (set `local.OriginLocation` _array_element)
        (bind _index (`self.ProperForLoop` (* _radius -1.0) _radius (`self.SpacingOnHeight`) true)
          (:`Loop`
            (set `local.Z` _index)
            (set `local.DiskRadius` (`KismetMathLibrary.Sqrt` (- (`KismetMathLibrary.Square` (`self.Radius`)) (`KismetMathLibrary.Square` (`local.Z`)))))
            (set `local.Height` (+ _originlocation_z (`local.Z`)))
            (bind _index_2 (`self.ProperForLoop` 0.0 (`local.DiskRadius`) (`self.Spacing`) true)
              (:`Loop`
                (bind _output_get (set `local.R` _index_2))
                (set `local.Circumference` (* _output_get (`KismetMathLibrary.GetPI`) 2.0))
                (bind _output_get_2 (set `local.PointCount` (`KismetMathLibrary.Max` 1 (`KismetMathLibrary.Round` (/ (`local.Circumference`) (`self.Spacing`))))))
                (for _index_3 (range _output_get_2)
                  (bind _output_get_3 (set `local.I` _index_3))
                  (set `local.Angle` (/ (* (`KismetMathLibrary.GetPI`) _output_get_3 2.0) (`local.PointCount`)))
                  (`self.AddGeneratedVector` (+ (`local.OriginLocation`) (`KismetMathLibrary.MakeVector` (* (`local.R`) (`KismetMathLibrary.Cos` (`local.Angle`))) (* (`local.R`) (`KismetMathLibrary.Sin` (`local.Angle`))) (`local.Z`)))))))))))))