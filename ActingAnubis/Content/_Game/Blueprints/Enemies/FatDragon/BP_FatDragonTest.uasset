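; Test flying enemy (Fat Dragon) that endlessly roams random airborne points inside a CPathVolume.
; An EQS query picks a destination from the best 25%, then an async volume pathfind builds the waypoint path, re-querying on pathfinding failure.
; Tick steers toward each waypoint with movement input and interpolated rotation, starting a new query when the path ends.
; Optional debug spheres and lines show targets, failures and the current waypoint.
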(event `self.ReceiveBeginPlay`
  (bind _returnvalue (`GameplayStatics.GetActorOfClass` "/Script/CPathfinding.CPathVolume"))
  (set `self.VoumeRightOne` _returnvalue)
  (`self.VoumeRightOne`
    (:`then`
      (bind _returnvalue_2 (`EnvQueryManager.RunEQSQuery` "/Game/_Game/Blueprints/AI/EQS/EQ_RandomLocationFlying.EQ_RandomLocationFlying" self "RandomBest25Pct" :!label _label))
      (add `EnvQueryInstanceBlueprintWrapper.OnQueryFinishedEvent` _returnvalue_2 (delegate `CustomEvent`)))
    (:`else`)))

(event `CustomEvent`
  (params (QueryInstance :type "EnvQueryInstanceBlueprintWrapper Object Reference") (QueryStatus :type "EEnvQueryStatus Enum" :default "Processing"))
  (switch `EEnvQueryStatus` QueryStatus
    (:`Success`
      (bind (_resultlocations _returnvalue) (`EnvQueryInstanceBlueprintWrapper.GetQueryResultsAsLocations` QueryInstance))
      (if _returnvalue
        (bind _output_get (set `self.EndLocation` (`|GetArrayItem` _resultlocations)))
        (`|ExecutionSequence`
          (:`then_0`
            (`self.DrawSphereAtLocationAndLineToId` _output_get (struct :`R` 1.0 :`G` 0.093247 :`A` 1.0) 20.0))
          (:`then_1`
            (bind _path (`CPathAsyncFindPath.FindPathAsync` (`self.VoumeRightOne`) (`self.K2_GetActorLocation`) _output_get)
              (:`Success`
                (set `self.CreatedPath` _path))
              (:`Failure`
                (`self.DrawSphereAtLocationAndLineToId` (`self.EndLocation`) (struct :`R` 1.0 :`B` 0.995726 :`A` 1.0) 20.0 2.0)
                (goto _label)))))))))

(event `self.ReceiveTick`
  (params (DeltaSeconds :type "Float (single-precision)"))
  (bind _worldlocation (break `CPathNode` (`|GetArrayItem` (`self.CreatedPath`) (`self.CurrentLocationIndex`))))
  (bind _returnvalue (`KismetMathLibrary.GetDirectionUnitVector` (`self.K2_GetActorLocation`) _worldlocation))
  (if (not (`KismetArrayLibrary.Array_IsEmpty` (`self.CreatedPath`)))
    (`self.DrawSphereAtLocationAndLineToId` _worldlocation (struct :`G` 0.533881 :`B` 1.0 :`A` 1.0) 0.0 3.0)
    (`self.AddMovementInput` _returnvalue)
    (`self.K2_SetActorRotation` (`KismetMathLibrary.RInterpTo` (`self.K2_GetActorRotation`) (`KismetMathLibrary.Conv_VectorToRotator` _returnvalue) DeltaSeconds 5.0))
    (if (`/Game/_Game/Blueprints/Library/BP_MathLibrary.DistanceBetweenVectorsWithinTolerance` (`self.K2_GetActorLocation`) _worldlocation 200.0)
      (bind _result (`/Engine/EditorBlueprintResources/StandardMacros.IncrementInt` (`self.CurrentLocationIndex`))
        (:`  `
          (if (not (`KismetArrayLibrary.Array_IsValidIndex` (`self.CreatedPath`) _result))
            (`KismetArrayLibrary.Array_Clear` (`self.CreatedPath`))
            (set `self.CurrentLocationIndex` 0)
            (goto _label)))))))

(fn `DrawSphereAtLocationAndLineToId`
  (params (Center :type "Vector Structure") (LineColor :type "LinearColor Structure") (Duration :type "Float (single-precision)") (Thickness :type "Float (single-precision)"))
  (if (`self.DrawDebug`)
    (`KismetSystemLibrary.DrawDebugSphere` Center 20.0 12 LineColor Duration Thickness)
    (`KismetSystemLibrary.DrawDebugLine` Center (`self.K2_GetActorLocation`) LineColor Duration Thickness)))

(fn `UserConstructionScript`)