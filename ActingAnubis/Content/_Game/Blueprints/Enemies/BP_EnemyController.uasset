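; AI controller for enemies that sets up each pawn's behavior tree and flags it as in combat.
; On possess, it runs the main tree from the pawn's BP_BehaviourTreeInfos component, or a default, and injects its combat and out-of-combat subtrees by gameplay tag.
; The first damage event or sighting of the player adds the InCombat status tag and disables sight sensing, with no reverse transition here.
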(event `self.ReceivePossess`
  (params (PossessedPawn :type "Pawn Object Reference"))
  (`self.SetupBehaviorTree` PossessedPawn)
  (`AbilityAsync_WaitGameplayEvent.WaitGameplayEventToActor` PossessedPawn (struct :`TagName` "Gameplay.Event.HealthComponent.Damage") true
    (:`EventReceived`
      (`AnubisAbilitySystemLibrary.AddStatusTags` (`self.K2_GetPawn`) (struct :`GameplayTags` (struct :`(TagName` "Status.ArtificialIntelligence.InCombat"))))
      (`AIPerceptionComponent.SetSenseEnabled` (`self.AIPerception`) "/Script/AIModule.AISense_Sight" false))))

(event `self.ReceiveBeginPlay`)

(event `self.AIPerception.OnTargetPerceptionUpdated`
  (params (Actor :type "Actor Object Reference") (Stimulus :type "AIStimulus Structure"))
  (if (and (== Actor (`GameplayStatics.GetPlayerCharacter` 0)) (`.bSuccessfullySensed` (break `AIStimulus` Stimulus)))
    (`AnubisAbilitySystemLibrary.AddStatusTags` (`self.K2_GetPawn`) (struct :`GameplayTags` (struct :`(TagName` "Status.ArtificialIntelligence.InCombat"))))
    (`AIPerceptionComponent.SetSenseEnabled` (`self.AIPerception`) "/Script/AIModule.AISense_Sight" false)))

(fn `PrintAbsenceOfComponentError`
  (params (Object :type "Object Object Reference"))
  (`KismetSystemLibrary.PrintText` (`|FormatText` "{Pawn} Does not have BP_BehaviourTreeInfos Component, Cannot properly Init Behavior Tree" (`KismetSystemLibrary.GetDisplayName` Object)) true true (struct :`R` 1.0 :`A` 1.0)))

(fn `SetupBehaviorTree`
  (params (PossessedPanw :type "Actor Object Reference"))
  (locals (InfoComponent :type "/Game/_Game/Blueprints/Enemies/BP_BehaviourTreeInfos Object Reference"))
  (bind _behaviortree (`self.BehaviorTree`))
  (bind _infocomponent (`local.InfoComponent`))
  (bind _mainbehaviortree (`/Game/_Game/Blueprints/Enemies/BP_BehaviourTreeInfos.MainBehaviorTree` (`local.InfoComponent`)))
  (bind _output_get (set `local.InfoComponent` (`self.GetComponentByClass` PossessedPanw "/Game/_Game/Blueprints/Enemies/BP_BehaviourTreeInfos.BP_BehaviourTreeInfos_C")))
  (`/Engine/EditorBlueprintResources/StandardMacros.IsValid` _output_get
    (:`Is Valid`
      (`|ExecutionSequence`
        (:`then_0`
          (`self.RunBehaviorTree` (select `bool` (`KismetSystemLibrary.IsValid` _mainbehaviortree) :`false` (`BehaviorTreeComponent.DefaultBehaviorTreeAsset` (`self.BehaviorTree`)) :`true` _mainbehaviortree)))
        (:`then_1`
          (`BehaviorTreeComponent.SetDynamicSubtree` _behaviortree (struct :`TagName` "ArtificialIntelligence.BehaviourTree.InjectionTag.Combat") (`/Game/_Game/Blueprints/Enemies/BP_BehaviourTreeInfos.BehaviourTreeForCombat` _infocomponent))
          (`BehaviorTreeComponent.SetDynamicSubtree` _behaviortree (struct :`TagName` "ArtificialIntelligence.BehaviourTree.InjectionTag.OutOfCombat") (`/Game/_Game/Blueprints/Enemies/BP_BehaviourTreeInfos.BehaviourTreeForOutOfCombat` _infocomponent)))))
    (:`Is Not Valid`
      (`self.PrintAbsenceOfComponentError` PossessedPanw))))

(fn `UserConstructionScript`)