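; BP_SimpleGravityCompnent is a component that applies simple gravity to its owner while it lacks the Status.Physics.IsSimulating tag.
; Each tick moves the owner down with a swept SetActorLocation at a constant speed set by GravityScale, without acceleration.
; After confirming a primitive root on BeginPlay, a self-rearming pair of gameplay tag waits disables tick when the tag is added and re-enables it on removal.
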(event `StartWaitingForImmovableTag`
  (bind _returnvalue (`self.GetOwner`))
  (`AbilityAsync_WaitGameplayTagAdded.WaitGameplayTagAddToActor` _returnvalue (struct :`TagName` "Status.Physics.IsSimulating") true
    (:`Added`
      (`self.SetComponentTickEnabled` false)
      (`AbilityAsync_WaitGameplayTagRemoved.WaitGameplayTagRemoveFromActor` _returnvalue (struct :`TagName` "Status.Physics.IsSimulating") true
        (:`Removed`
          (`self.SetComponentTickEnabled` true)
          (`self.StartWaitingForImmovableTag`))))))

(event `self.ReceiveBeginPlay`
  (bind _asprimitive_component (cast `PrimitiveComponent` (`Actor.RootComponent` (`self.GetOwner`))))
  (set `self.PrimitiveComponentRoot` _asprimitive_component)
  (`self.SetComponentTickEnabled` true)
  (`self.StartWaitingForImmovableTag`))

(event `self.ReceiveTick`
  (params (DeltaSeconds :type "Float (single-precision)"))
  (bind _returnvalue (`self.GetOwner`))
  (`Actor.K2_SetActorLocation` _returnvalue (+ (`Actor.K2_GetActorLocation` _returnvalue) (* (`KismetMathLibrary.Vector_Down`) (`self.GravityScale`) DeltaSeconds)) true false))