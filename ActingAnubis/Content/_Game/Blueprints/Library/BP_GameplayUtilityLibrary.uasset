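; BP_GameplayUtilityLibrary is a Blueprint function library of shared gameplay helpers for camera, player, tag and socket lookups.
; Camera and player helpers default to player index 0 and can return forward-scaled locations.
; Tag helpers trim dotted prefixes, turning Animation.Sections child tags into montage-style section names.
; A blackboard key-to-location/actor function is an unwired reference, marked to be copied because it is not possible in Blueprint.
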(fn `GetAnimationSectionNameFromTag`
  (params (GameplayTag :type "GameplayTag Structure (by ref)"))
  (returns (bSuccess :type Boolean) (SectionName :type Name))
  (if (and (`BlueprintGameplayTagLibrary.MatchesTag` GameplayTag (struct :`TagName` "Animation.Sections")) (not (`BlueprintGameplayTagLibrary.MatchesTag` GameplayTag (struct :`TagName` "Animation.Sections") true)))
    (return true (`KismetStringLibrary.Conv_StringToName` (`self.SplitTagName` GameplayTag 1 2 (`local.__WorldContext`))))
    (else
      (return false "None"))))

(fn `GetAttackSocketName`
  (returns (SocketName :type Name))
  (return "ShootProjectileSpawnLocation"))

(fn `GetCameraForwardVector`
  (params (OptionalController :type "Controller Object Reference"))
  (returns (ReturnValue :type "Vector Structure"))
  (locals (Controller :type "Controller Object Reference"))
  (bind _output_get (set `local.Controller` (select `bool` (`KismetSystemLibrary.IsValid` OptionalController) :`false` (`GameplayStatics.GetPlayerController` (`local.__WorldContext`)) :`true` OptionalController :!type "Controller Object Reference")))
  (return (`Actor.GetActorForwardVector` _output_get)))

(fn `GetCameraLocation`
  (params (OptionalPlayerController :type "PlayerController Object Reference"))
  (returns (ReturnValue :type "Vector Structure"))
  (locals (PlayerController :type "PlayerController Object Reference"))
  (bind _output_get (set `local.PlayerController` (select `bool` (`KismetSystemLibrary.IsValid` OptionalPlayerController) :`false` (`GameplayStatics.GetPlayerController` (`local.__WorldContext`)) :`true` OptionalPlayerController)))
  (return (`PlayerCameraManager.GetCameraLocation` (`PlayerController.PlayerCameraManager` _output_get))))

(fn `GetCameraRotation`
  (params (OptionalController :type "Controller Object Reference"))
  (returns (ReturnValue :type "Rotator Structure"))
  (locals (Controller :type "Controller Object Reference"))
  (bind _output_get (set `local.Controller` (select `bool` (`KismetSystemLibrary.IsValid` OptionalController) :`false` (`GameplayStatics.GetPlayerController` (`local.__WorldContext`)) :`true` OptionalController :!type "Controller Object Reference")))
  (return (`Controller.GetControlRotation` _output_get)))

(fn `GetCameraTransformInfo`
  (params (OptionalPlayerController :type "PlayerController Object Reference") (ForwardScale :type "Float (double-precision)"))
  (returns (CameraLocation :type "Vector Structure") (CameraForwardVector :type "Vector Structure") (CameraRotation :type "Rotator Structure") (CameraLocationWithForwardScaled :type "Vector Structure"))
  (locals (PlayerController :type "PlayerController Object Reference") (`Camera Location` :type "Vector Structure" :default (0.0 0.0 0.0)) (`Camera Forward Vector` :type "Vector Structure" :default (0.0 0.0 0.0)))
  (bind _output_get (set `local.PlayerController` (select `bool` (`KismetSystemLibrary.IsValid` OptionalPlayerController) :`false` (`GameplayStatics.GetPlayerController` (`local.__WorldContext`)) :`true` OptionalPlayerController)))
  (set `local.Camera Location` (`PlayerCameraManager.GetCameraLocation` (`PlayerController.PlayerCameraManager` _output_get)))
  (set `local.Camera Forward Vector` (`Actor.GetActorForwardVector` _output_get))
  (return (`local.Camera Location`) (`local.Camera Forward Vector`) (`Controller.GetControlRotation` _output_get) (+ (`local.Camera Location`) (* (`local.Camera Forward Vector`) (`local.ForwardScale`)))))

(fn `GetLocationAndActorFromKey NOT POSSIBLE IN BP, COPY LOGIC`
  (params (BlackboardKeySelector :type "BlackboardKeySelector Structure (by ref)"))
  (returns (bSuccess :type Boolean) (OutActor :type "Actor Object Reference") (ActorIsValid :type Boolean) (OutLocation :type "Vector Structure"))
  (locals (TargetActor :type "Actor Object Reference") (TargetLocation :type "Vector Structure")))

(fn `GetPlayerLocationWithForwardScale`
  (params (OptionalController :type "Controller Object Reference") (OptionalPlayerActor :type "Actor Object Reference") (ForwardScale :type "Float (single-precision)"))
  (returns (OutPlayerLocation :type "Vector Structure") (LocationWithForwardScale :type "Vector Structure"))
  (locals (PlayerActor :type "Actor Object Reference") (PlayerLocation :type "Vector Structure" :default (0.0 0.0 0.0)))
  (bind _optionalplayeractor (`local.OptionalPlayerActor`))
  (bind _output_get (set `local.PlayerActor` (select `bool` (`KismetSystemLibrary.IsValid` _optionalplayeractor) :`false` (`GameplayStatics.GetPlayerPawn` (`local.__WorldContext`)) :`true` _optionalplayeractor :!type "Actor Object Reference")))
  (bind _output_get_2 (set `local.PlayerLocation` (`Actor.K2_GetActorLocation` _output_get)))
  (return _output_get_2 (+ _output_get_2 (* (`Actor.GetActorForwardVector` _output_get) (`local.ForwardScale`)))))

(fn `SplitTagName`
  (params (GameplayTag :type "GameplayTag Structure (by ref)") (FirstIndex :type Integer :default 1) (LastIndex :type Integer :default 2))
  (returns (ShortNameString :type String) (ShortNameText :type Text))
  (locals (TagName :type String))
  (bind _tagname (`local.TagName`))
  (bind (_lefts _rights _returnvalue) (`KismetStringLibrary.Split` (`local.TagName`) "."))
  (set `local.TagName` (`KismetStringLibrary.Conv_NameToString` (`BlueprintGameplayTagLibrary.GetTagName` GameplayTag)))
  (for _ (range (`local.FirstIndex`) (+ (`local.LastIndex`) 1))
    (if _returnvalue
      (set `local.TagName` _rights)
      (else
        (break))))
  (return _tagname (`KismetTextLibrary.Conv_StringToText` _tagname)))