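; Blueprint function library of shared gameplay helpers for physics pushes, health, abilities, tag-driven animation lookup and visibility checks.
; Damage, healing, max-health changes and pushes send gameplay events; health getters read BP_HealthComponent directly.
; Pushes also apply velocity-change impulses unless the target is tagged as handling them manually.
; Animations resolve from Identifier-tag data table rows via tag queries, while visibility uses line traces to the target's center, top and bottom.
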(fn `ActorIsVisible`
  (params (`ActorInsigator (Origin)` :type "Actor Object Reference") (`ActorTarget (ToSee)` :type "Actor Object Reference") (ZBoundsOffset :type "Float (double-precision)" :default 25.0) (`bShootFromCamera?` :type Boolean) (DrawDebugType :type "EDrawDebugTrace Enum" :default "None") (TraceChannel :type "ETraceTypeQuery Enum" :default "TraceTypeQuery1") (OptionalIgnoreActors :type "Array of Actor Object Reference"))
  (returns (ReturnValue :type Boolean))
  (locals (IgnoreActors :type "Array of Actor Object Reference") (OriginLocation :type "Vector Structure") (TargetLocation :type "Vector Structure") (ZBounds :type "Float (double-precision)"))
  (bind (_origin _boxextent) (`Actor.GetActorBounds` `ActorTarget (ToSee)` false false))
  (bind _output_get (set `local.IgnoreActors` OptionalIgnoreActors))
  (`KismetArrayLibrary.Array_Append` _output_get (`|MakeArray` `ActorInsigator (Origin)` `ActorTarget (ToSee)`))
  (set `local.OriginLocation` (select `bool` (`local.bShootFromCamera?`) :`false` (`Actor.K2_GetActorLocation` `ActorInsigator (Origin)`) :`true` (`/Game/_Game/Blueprints/Library/BP_GameplayUtilityLibrary.GetCameraLocation` null (`local.__WorldContext`))))
  (set `local.TargetLocation` _origin)
  (set `local.ZBounds` (- (.z _boxextent) (`local.ZBoundsOffset`)))
  (`|ExecutionSequence`
    (:`then_0`
      (bind (_outhit _returnvalue) (`KismetSystemLibrary.LineTraceSingle` (`local.__WorldContext`) (`local.OriginLocation`) (`local.TargetLocation`) (`local.TraceChannel`) false (`local.IgnoreActors`) (`local.DrawDebugType`)))
      (if (not _returnvalue)
        (return true)))
    (:`then_1`
      (bind (_outhit_2 _returnvalue_2) (`KismetSystemLibrary.LineTraceSingle` (`local.__WorldContext`) (`local.OriginLocation`) (+ (`local.TargetLocation`) (`KismetMathLibrary.MakeVector` 0.0 0.0 (`local.ZBounds`))) (`local.TraceChannel`) false (`local.IgnoreActors`) (`local.DrawDebugType`)))
      (if (not _returnvalue_2)
        (return true)))
    (:`then_2`
      (bind (_outhit_3 _returnvalue_3) (`KismetSystemLibrary.LineTraceSingle` (`local.__WorldContext`) (`local.OriginLocation`) (- (`local.TargetLocation`) (`KismetMathLibrary.MakeVector` 0.0 0.0 (`local.ZBounds`))) (`local.TraceChannel`) false (`local.IgnoreActors`) (`local.DrawDebugType`)))
      (if (not _returnvalue_3)
        (return true)))
    (:`then_3`
      (return false))))

(fn `DealDamageToActor`
  (params (Actor :type "Actor Object Reference") (Instigator :type "Actor Object Reference") (Damage :type "Float (double-precision)"))
  (`AbilitySystemBlueprintLibrary.SendGameplayEventToActor` Actor (struct :`TagName` "Gameplay.Event.HealthComponent.Damage") (make `GameplayEventData` :`Instigator` Instigator :`EventMagnitude` Damage)))

(fn `ExecutePushOnPushableObject`
  (params (ImpulseTargetActor :type "Actor Object Reference") (PhysicsComponent :type "PrimitiveComponent Object Reference") (Instigator :type "Actor Object Reference") (DirectionImpulseNorm :type "Vector Structure") (ImpulseStrength :type "Float (double-precision)"))
  (bind _physicscomponent (`local.PhysicsComponent`))
  (`|ExecutionSequence`
    (:`then_0`
      (`/Engine/EditorBlueprintResources/StandardMacros.IsValid` _physicscomponent
        (:`Is Valid`
          (bind _returnvalue (`AnubisAbilitySystemLibrary.HasMatchingGameplayTag` (`local.ImpulseTargetActor`) (struct :`TagName` "Status.Physics.Push.HandlesManually")))
          (if (and (not _returnvalue) (`SceneComponent.IsSimulatingPhysics` _physicscomponent "None"))
            (`PrimitiveComponent.AddImpulse` (`local.PhysicsComponent`) (* (`local.DirectionImpulseNorm`) (`local.ImpulseStrength`)) "None" true)))))
    (:`then_1`
      (`AbilitySystemBlueprintLibrary.SendGameplayEventToActor` (`local.ImpulseTargetActor`) (struct :`TagName` "Gameplay.Event.Physics.Impulse") (make `GameplayEventData` :`Instigator` (`local.Instigator`) :`Target` (`local.ImpulseTargetActor`) :`EventMagnitude` (`local.ImpulseStrength`))))))

(fn `GetActorHealth`
  (params (Target :type "Actor Object Reference"))
  (returns (bSuccess :type Boolean) (CurrentHealth :type "Float (double-precision)"))
  (bind _returnvalue (`Actor.GetComponentByClass` Target "/Game/_Game/Blueprints/BP_HealthComponent.BP_HealthComponent_C"))
  (`/Engine/EditorBlueprintResources/StandardMacros.IsValid` _returnvalue
    (:`Is Valid`
      (return true (`/Game/_Game/Blueprints/BP_HealthComponent.GetHealth` _returnvalue)))
    (:`Is Not Valid`
      (return false 0.0))))

(fn `GetActorHealthStats`
  (params (Target :type "Actor Object Reference"))
  (returns (bSuccess :type Boolean) (CurrentHealth :type "Float (double-precision)") (MaxHealth :type "Float (double-precision)"))
  (bind _returnvalue (`Actor.GetComponentByClass` Target "/Game/_Game/Blueprints/BP_HealthComponent.BP_HealthComponent_C"))
  (bind (_currenthealth _maxhealth) (`/Game/_Game/Blueprints/BP_HealthComponent.GetHealthStats` _returnvalue))
  (`/Engine/EditorBlueprintResources/StandardMacros.IsValid` _returnvalue
    (:`Is Valid`
      (return true _currenthealth _maxhealth))
    (:`Is Not Valid`
      (return false 0.0 0.0))))

(fn `GetActorMaxHealth`
  (params (Target :type "Actor Object Reference"))
  (returns (bSuccess :type Boolean) (MaxHealth :type "Float (double-precision)"))
  (bind _returnvalue (`Actor.GetComponentByClass` Target "/Game/_Game/Blueprints/BP_HealthComponent.BP_HealthComponent_C"))
  (`/Engine/EditorBlueprintResources/StandardMacros.IsValid` _returnvalue
    (:`Is Valid`
      (return true (`/Game/_Game/Blueprints/BP_HealthComponent.GetMaxHealth` _returnvalue)))
    (:`Is Not Valid`
      (return false 0.0))))

(fn `GetAnimationByIdentifier`
  (params (OwnedTags :type "GameplayTagContainer Structure (by ref)") (ExtraTagsParams :type "GameplayTagContainer Structure"))
  (returns (bSuccess :type Boolean) (AnimMontage :type "AnimMontage Object Reference") (SectionName :type Name))
  (locals (FilteredTags :type "GameplayTagContainer Structure") (QueryParamTags :type "GameplayTagContainer Structure") (CurrentAnimQuery :type "/Game/_Game/Animations/AnimationByIdentifier/S_AnimationByQuery Structure"))
  (bind ((`AnimMontage_5_D58673EB49E5F88C26E3519A3CBBE951` _animmontage) (`Section_8_72F44CE04F37CBF34ED0F78F7F8A58CE` _section)) (break `/Game/_Game/Animations/AnimationByIdentifier/S_AnimationByQuery` (`local.CurrentAnimQuery`)))
  (bind (_bsuccess _identifiertag) (`self.GetIdentifierTag` OwnedTags (`local.__WorldContext`)))
  (if _bsuccess
    (bind _returnvalue (`|GetDataTableRow` "/Game/_Game/Animations/AnimationByIdentifier/DT_AnimationsByIdentifier.DT_AnimationsByIdentifier" (`BlueprintGameplayTagLibrary.GetTagName` _identifiertag))
      (:`then`
        (`|ExecutionSequence`
          (:`then_0`
            (bind _output_get (set `local.QueryParamTags` (`local.OwnedTags`)))
            (`BlueprintGameplayTagLibrary.AppendGameplayTagContainers` _output_get (`local.ExtraTagsParams`)))
          (:`then_1`
            (for _array_element (`.Query_7_729B21974B1EB422B5A900A44A2894E3` (break `/Game/_Game/Animations/AnimationByIdentifier/S_AnimationsByIdentifier` _returnvalue))
              (bind _output_get_2 (set `local.CurrentAnimQuery` _array_element))
              (bind ((`TagQuery_2_5F8E56F44C36D7BA7BA659A3C04FC922` _tagquery) (`SectionTag_11_FC0AECEA4BC22867F42D84996E79EE59` _sectiontag)) (break `/Game/_Game/Animations/AnimationByIdentifier/S_AnimationByQuery` _output_get_2))
              (if (`BlueprintGameplayTagLibrary.DoesContainerMatchTagQuery` (`local.QueryParamTags`) _tagquery)
                (bind (_bsuccess_2 _sectionname) (`/Game/_Game/Blueprints/Library/BP_GameplayUtilityLibrary.GetAnimationSectionNameFromTag` _sectiontag (`local.__WorldContext`)))
                (return true _animmontage (`KismetMathLibrary.SelectName` _sectionname _section _bsuccess_2))))
            (return false null "None"))))
      (:`RowNotFound`
        (return false null "None")))
    (else
      (return false null "None"))))

(fn `GetIdentifierTag`
  (params (OwnedTags :type "GameplayTagContainer Structure (by ref)"))
  (returns (bSuccess :type Boolean) (IdentifierTag :type "GameplayTag Structure"))
  (locals (FilteredTags :type "GameplayTagContainer Structure") (OutTag :type "GameplayTag Structure"))
  (if (`KismetArrayLibrary.Array_IsNotEmpty` (`BlueprintGameplayTagLibrary.BreakGameplayTagContainer` OwnedTags))
    (bind _returnvalue (`AnubisAbilitySystemLibrary.FilterTagContainer` OwnedTags (`BlueprintGameplayTagLibrary.MakeGameplayTagContainerFromTag` (struct :`TagName` "Identifier"))))
    (bind _output_get (set `local.FilteredTags` _returnvalue))
    (bind _gameplaytags (`BlueprintGameplayTagLibrary.BreakGameplayTagContainer` _output_get))
    (if (`KismetArrayLibrary.Array_IsNotEmpty` _gameplaytags)
      (if (> (`KismetArrayLibrary.Array_Length` _gameplaytags) 1)
        (for _array_element (`BlueprintGameplayTagLibrary.BreakGameplayTagContainer` _output_get)
          (bind _output_get_2 (set `local.OutTag` _array_element))
          (if (not (`BlueprintGameplayTagLibrary.MatchesTag` _output_get_2 (struct :`TagName` "Identifier") true))
            (`KismetSystemLibrary.PrintText` (`local.__WorldContext`) (`|FormatText` "Tried to get Identifier tag from an actor with Multiple Identifiers, Only first one will be used : {tag}" (`BlueprintGameplayTagLibrary.GetTagName` (`local.OutTag`))) true true (struct :`R` 1.0 :`A` 1.0) 10.0)
            (return true (`local.OutTag`))))
        (return false)
        (else
          (bind _output_get_3 (set `local.OutTag` (`|GetArrayItem` _gameplaytags)))
          (return (not (`BlueprintGameplayTagLibrary.MatchesTag` _output_get_3 (struct :`TagName` "Identifier") true)) _output_get_3)))
      (else
        (return false)))
    (else
      (return false))))

(fn `HealActor`
  (params (Actor :type "Actor Object Reference") (Instigator :type "Actor Object Reference") (HealingAmout :type "Float (double-precision)"))
  (`AbilitySystemBlueprintLibrary.SendGameplayEventToActor` Actor (struct :`TagName` "Gameplay.Event.HealthComponent.Healing") (make `GameplayEventData` :`Instigator` Instigator :`EventMagnitude` HealingAmout)))

(fn `ModifyMaxHealthOnActor`
  (params (Actor :type "Actor Object Reference") (Instigator :type "Actor Object Reference") (DeltaHealth :type "Float (double-precision)"))
  (`AbilitySystemBlueprintLibrary.SendGameplayEventToActor` Actor (struct :`TagName` "Gameplay.Event.HealthComponent.MaxHealth.Modify") (make `GameplayEventData` :`Instigator` Instigator :`EventMagnitude` DeltaHealth)))

(fn `RemoveAbilitySelf`
  (params (ASC :type "AbilitySystemComponent Object Reference") (ThisAbility :type "Object Object Reference"))
  (bind _outabilityhandles (`AbilitySystemComponent.GetAllAbilities` ASC))
  (for _array_element _outabilityhandles
    (if (== (`.ReturnValue` (`AbilitySystemBlueprintLibrary.GetGameplayAbilityFromSpecHandle` ASC _array_element)) ThisAbility)
      (`AbilitySystemComponent.ClearAbility` ASC _array_element)
      (return))))