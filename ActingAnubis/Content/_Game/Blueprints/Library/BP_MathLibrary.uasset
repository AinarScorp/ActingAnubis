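; BP_MathLibrary is a Blueprint library of small vector math helpers.
; DistanceBetweenVectorsWithinTolerance tests whether two points lie within a tolerance, optionally ignoring Z, by comparing squared distance to squared tolerance.
; GetUnitDirection(Actors) returns the unit direction from one actor's location to another's.
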(fn `DistanceBetweenVectorsWithinTolerance`
  (params (V1 :type "Vector Structure") (V2 :type "Vector Structure") (Tolerance :type "Float (double-precision)") (bIgnoreZ :type Boolean))
  (returns (ReturnValue :type Boolean))
  (bind _returnvalue (`KismetMathLibrary.Square` (`local.Tolerance`)))
  (return (select `bool` (`local.bIgnoreZ`) :`false` (<= (`KismetMathLibrary.Vector_DistanceSquared` V1 V2) _returnvalue) :`true` (<= (`KismetMathLibrary.Vector_Distance2DSquared` V1 V2) _returnvalue))))

(fn `GetUnitDirection(Actors)`
  (params (From :type "Actor Object Reference") (To :type "Actor Object Reference"))
  (returns (ReturnValue :type "Vector Structure"))
  (return (`KismetMathLibrary.GetDirectionUnitVector` (`Actor.K2_GetActorLocation` From) (`Actor.K2_GetActorLocation` To))))