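; Anim notify that sends a configurable gameplay event tag to the animated mesh's owning actor.
; It sends only when a valid Game Mode exists, which excludes network clients and returns false there.
; The notify's display name is a shortened form of the tag, cut between configurable start and end indices.
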(fn `GetNotifyName`
  (returns (ReturnValue :type String))
  (return (`/Game/_Game/Blueprints/Library/BP_GameplayUtilityLibrary.SplitTagName` (`self.EventTag`) (`self.ShortenTag_Start`) (`self.ShortenTag_End`))))

(fn `Received_Notify`
  (params (MeshComp :type "SkeletalMeshComponent Object Reference") (Animation :type "AnimSequenceBase Object Reference") (EventReference :type "AnimNotifyEventReference Structure (by ref)"))
  (returns (ReturnValue :type Boolean))
  (`/Engine/EditorBlueprintResources/StandardMacros.IsValid` (`GameplayStatics.GetGameMode`)
    (:`Is Valid`
      (`AbilitySystemBlueprintLibrary.SendGameplayEventToActor` (`ActorComponent.GetOwner` MeshComp) (`self.EventTag`))
      (return true))
    (:`Is Not Valid`
      (return false))))