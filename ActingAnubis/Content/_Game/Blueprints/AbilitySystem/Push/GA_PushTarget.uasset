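; Gameplay ability that pushes its avatar away from an event's instigator by launching the skeletal mesh with physics.
; Activation applies a magnitude-scaled impulse, disables root collision and starts a simulation timer.
; A tick task then waits for the mesh to slow, moves the actor to it using the cached relative transform, and rotates toward upright on the traced floor normal.
; Uncancelled endings restore root collision and stop physics.
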(event `self.K2_OnEndAbility`
  (params (bWasCancelled :type Boolean))
  (set `self.IsFlipping` false)
  (if (`self.LaunchedSuccessfully`)
    (if (not bWasCancelled)
      (`self.HandleRootComponentCollision` (`self.CachedCollisionSetting`))
      (`self.ToggleSimulatingPhysics` false)
      (set `self.LaunchedSuccessfully` false))))

(event `self.K2_ActivateAbilityFromEvent`
  (params (EventData :type "GameplayEventData Structure (by ref)"))
  (bind _bsuccess (`self.LaunchSkeletalMesh` EventData))
  (if _bsuccess
    (set `self.LaunchedSuccessfully` true)
    (`self.HandleRootComponentCollision` "NoCollision" true)
    (`self.StartDelayTimer`)
    (else
      (`self.K2_CancelAbility`))))

(event `StartWaitingForRotatingBackTime`
  (`KismetSystemLibrary.K2_ClearAndInvalidateTimerHandle` (`self.DelayTimer`))
  (bind (_asynctaskproxy _deltatime) (`AnubisAbilityTask_TickTask.CreateTickTask` null)
    (:`then`
      (set `self.TickTask` _asynctaskproxy))
    (:`OnUpdate`
      (set `self.Delta Time` _deltatime)
      (if (`self.ShouldStartRotatingBack`)
        (`|ExecutionSequence`
          (:`then_0`
            (if (not (`self.IsFlipping`))
              (`|ExecutionSequence`
                (:`then_0`
                  (`self.ToggleSimulatingPhysics` false)
                  (`self.HandleRootComponentCollision` "NoCollision"))
                (:`then_1`
                  (bind _output_get (set `self.SkeletalMeshTransform` (`SceneComponent.K2_GetComponentToWorld` (`self.SkeletalMeshComponent`))))
                  (`self.DrawDebugCoordinates` _output_get)
                  (`|ExecutionSequence`
                    (:`then_0`
                      (bind _impactnormal (`self.FindFloorNormal`))
                      (set `self.Impact Normal` _impactnormal)
                      (set `self.ActorDesiredForward` (`KismetMathLibrary.Normal` (`KismetMathLibrary.ProjectVectorOnToPlane` (`Actor.GetActorForwardVector` (`self.GetAvatarActorFromActorInfo`)) (`self.Impact Normal`)))))
                    (:`then_1`
                      (`self.CombineMeshWithActorOrigin`)))))))
          (:`then_1`
            (set `self.IsFlipping` true))
          (:`then_2`
            (`self.RotateBackToFaceUp`)
            (`self.K2_EndAbility`)))))))

(event `self.BP_OnGiveAbility`
  (params (ActorInfo :type "GameplayAbilityActorInfo Structure (by ref)"))
  (bind (_owneractor _avataractor) (break `GameplayAbilityActorInfo` ActorInfo))
  (bind _asprimitive_component (cast `PrimitiveComponent` (`Actor.RootComponent` _avataractor)))
  (`PrimitiveComponent.SetCollisionResponseToChannel` _asprimitive_component "ECC_GameTraceChannel1" "ECR_Overlap")
  (set `self.RelativeTransform` (`SceneComponent.GetRelativeTransform` (`Actor.GetComponentByClass` _avataractor "/Script/Engine.SkeletalMeshComponent"))))

(fn `CombineMeshWithActorOrigin`
  (bind (_returnvalue _rotation) (`self.GetLocationAndRotationOfAdjustTransforms`))
  (`Actor.K2_SetActorLocationAndRotation` (`self.GetAvatarActorFromActorInfo`) _returnvalue _rotation false true)
  (`SceneComponent.K2_SetWorldLocationAndRotation` (`self.SkeletalMeshComponent`) (+ (.location (`self.SkeletalMeshTransform`)) (`self.OffGroundOffset`)) (.rotation (`self.SkeletalMeshTransform`)) false true))

(fn `DrawDebugArrow`
  (params (LineStart :type "Vector Structure") (LineEnd :type "Vector Structure") (ArrowSize :type "Float (single-precision)" :default 2.0) (LineColor :type "LinearColor Structure" :default (struct :`R` 0.909835 :`B` 1.0 :`A` 1.0)) (Thickness :type "Float (single-precision)" :default 10.0))
  (if (`|EnumInequality` (`self.Draw Debug Type`))
    (`KismetSystemLibrary.DrawDebugArrow` LineStart LineEnd ArrowSize LineColor 999.0 Thickness)))

(fn `DrawDebugCoordinates`
  (params (InTransform :type "Transform Structure (by ref)"))
  (bind (_returnvalue _rotation) (`self.GetLocationAndRotationOfAdjustTransforms`))
  (if (`|EnumInequality` (`self.Draw Debug Type`))
    (`KismetSystemLibrary.DrawDebugCoordinateSystem` (.location InTransform) (.rotation InTransform) 250.0 9999.0 1.0)
    (`KismetSystemLibrary.DrawDebugCoordinateSystem` _returnvalue _rotation 250.0 9999.0 5.0)))

(fn `FindFloorNormal`
  (returns (ImpactNormal :type "Vector Structure"))
  (bind _returnvalue (`self.GetLocationAndRotationOfAdjustTransforms`))
  (bind _outhit (`KismetSystemLibrary.LineTraceSingle` _returnvalue (+ _returnvalue (* (`KismetMathLibrary.Vector_Down`) 100000.0)) "TraceTypeQuery1" false (`|MakeArray` (`self.GetAvatarActorFromActorInfo`)) (`self.Draw Debug Type`) true (struct :`R` 1.0 :`A` 1.0) (struct :`G` 1.0 :`A` 1.0) 99.0))
  (return (`.ImpactNormal` (`GameplayStatics.BreakHitResult` _outhit))))

(fn `GetLocationAndRotationOfAdjustTransforms`
  (returns (ReturnValue :type "Vector Structure") (Rotation :type "Rotator Structure"))
  (bind _rotation (.rotation (`self.SkeletalMeshTransform`)))
  (return (+ (- (.location (`self.SkeletalMeshTransform`)) (`KismetMathLibrary.GreaterGreater_VectorRotator` (.location (`self.RelativeTransform`)) _rotation)) (`self.OffGroundOffset`)) (`KismetMathLibrary.Quat_Rotator` (* (`KismetMathLibrary.Conv_RotatorToQuaternion` _rotation) (`KismetMathLibrary.Quat_Inversed` (`KismetMathLibrary.Conv_RotatorToQuaternion` (.rotation (`self.RelativeTransform`))))))))

(fn `HandleRootComponentCollision`
  (params (NewCollisionType :type "ECollisionEnabled Enum" :default "NoCollision") (CacheCollisionSetting :type Boolean))
  (bind _asshape_component (cast `ShapeComponent` (`Actor.RootComponent` (`self.GetAvatarActorFromActorInfo`))))
  (`|ExecutionSequence`
    (:`then_0`
      (if (`local.CacheCollisionSetting`)
        (set `self.CachedCollisionSetting` (`PrimitiveComponent.GetCollisionEnabled` _asshape_component))))
    (:`then_1`
      (`PrimitiveComponent.SetCollisionEnabled` _asshape_component NewCollisionType))))

(fn `K2_ShouldAbilityRespondToEvent`
  (params (ActorInfo :type "GameplayAbilityActorInfo Structure") (Payload :type "GameplayEventData Structure"))
  (returns (ReturnValue :type Boolean))
  (return (`KismetSystemLibrary.IsValid` (`.Instigator` (break `GameplayEventData` Payload)))))

(fn `LaunchSkeletalMesh`
  (params (GameplayEventData :type "GameplayEventData Structure (by ref)"))
  (returns (bSuccess :type Boolean))
  (bind ((`Instigator` _instigator) (`EventMagnitude` _eventmagnitude)) (break `GameplayEventData` GameplayEventData))
  (`self.SkeletalMeshComponent`
    (:`then`
      _)
    (:`else`
      (bind _output_get (set `self.SkeletalMeshComponent` (`Actor.GetComponentByClass` (`self.GetAvatarActorFromActorInfo`) "/Script/Engine.SkeletalMeshComponent")))
      (`/Engine/EditorBlueprintResources/StandardMacros.IsValid` _output_get
        (:`Is Valid`
          _)
        (:`Is Not Valid`
          (return false)))))
  (`self.ToggleSimulatingPhysics` true)
  (`SkeletalMeshComponent.AddImpulseToAllBodiesBelow` (`self.SkeletalMeshComponent`) (* (+ (`/Game/_Game/Blueprints/Library/BP_MathLibrary.GetUnitDirection(Actors)` _instigator (`self.GetAvatarActorFromActorInfo`)) (0.0 0.0 0.2)) (* _eventmagnitude 0.5)) "None" true true)
  (return true))

(fn `RotateBackToFaceUp`
  (bind _actordesiredforward (`self.ActorDesiredForward`))
  (bind _actordesiredforward_2 (`self.ActorDesiredForward`))
  (`Actor.K2_SetActorRotation` (`self.GetAvatarActorFromActorInfo`) (`KismetMathLibrary.RInterpTo` (`Actor.K2_GetActorRotation` (`self.GetAvatarActorFromActorInfo`)) (`KismetMathLibrary.MakeRotationFromAxes` _actordesiredforward_2 (`KismetMathLibrary.Cross_VectorVector` (`self.Impact Normal`) _actordesiredforward_2) (`self.Impact Normal`)) (`self.Delta Time`) 1.0) false)
  (if (> (`KismetMathLibrary.Dot_VectorVector` (`Actor.GetActorForwardVector` (`self.GetAvatarActorFromActorInfo`)) (`self.ActorDesiredForward`)) 0.95)
    (`Actor.K2_SetActorRotation` (`self.GetAvatarActorFromActorInfo`) (`KismetMathLibrary.MakeRotationFromAxes` _actordesiredforward (`KismetMathLibrary.Cross_VectorVector` (`self.Impact Normal`) _actordesiredforward) (`self.Impact Normal`)) false)))

(fn `ShouldStartRotatingBack`
  (returns (ReturnValue :type Boolean))
  (return (or (`self.IsFlipping`) (<= (`KismetMathLibrary.VSize` (`SceneComponent.GetComponentVelocity` (`self.SkeletalMeshComponent`))) 100.0))))

(fn `StartDelayTimer`
  (bind _delaytimer (`self.DelayTimer`))
  (if (`KismetSystemLibrary.K2_IsValidTimerHandle` _delaytimer)
    (`KismetSystemLibrary.K2_ClearAndInvalidateTimerHandle` _delaytimer))
  (bind _returnvalue (`KismetSystemLibrary.K2_SetTimerDelegate` (`|CreateDelegate` :!event `StartWaitingForRotatingBackTime`) (`self.SimulatePhysicsTime`)))
  (set `self.DelayTimer` _returnvalue))

(fn `ToggleSimulatingPhysics`
  (params (bNewSimulate :type Boolean))
  (bind _skeletalmeshcomponent (`self.SkeletalMeshComponent`))
  (`PrimitiveComponent.SetSimulatePhysics` _skeletalmeshcomponent bNewSimulate)
  (`PrimitiveComponent.SetCollisionEnabled` _skeletalmeshcomponent (select `bool` bNewSimulate :`false` "NoCollision" :`true` "QueryAndPhysics" :!type "ECollisionEnabled Enum"))
  (return))