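; Gameplay ability that lets the caster push objects in front of them along the camera's forward direction.
; On activation, a multi box trace, oriented to the camera and offset ahead of the avatar, gathers candidate hits.
; Each hit with a valid actor that passes a camera-based visibility check receives a fixed-strength impulse on its hit component.
; The ability ends once the hits are processed.
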(event `self.K2_ActivateAbility`
  (bind _outhits (`self.GetPushableObjectsWithinReach`))
  (for _array_element _outhits
    (bind _returnvalue (`self.TargetCanBePushed` _array_element))
    (if _returnvalue
      (bind (_bblockinghit _binitialoverlap _time _distance _location _impactpoint _normal _impactnormal _physmat _hitactor _hitcomponent) (`GameplayStatics.BreakHitResult` _array_element))
      (`/Game/_Game/Blueprints/Library/BP_GameplayLibrary.ExecutePushOnPushableObject` _hitactor _hitcomponent (`self.GetAvatarActorFromActorInfo`) (`/Game/_Game/Blueprints/Library/BP_GameplayUtilityLibrary.GetCameraForwardVector` (`self.GetPlayerControllerFromActorInfo`)) 10000.0)))
  (`self.K2_EndAbility`))

(fn `GetPushableObjectsWithinReach`
  (returns (OutHits :type "Array of HitResult Structure"))
  (bind (_starttracelocation _endtracelocation _orientation) (`self.GetTraceParams`))
  (bind _outhits (`KismetSystemLibrary.BoxTraceMulti` :`Start` _starttracelocation :`End` _endtracelocation :`HalfSize` (`self.Half Size`) :`Orientation` _orientation :`TraceChannel` "TraceTypeQuery3" :`DrawDebugType` (`self.Draw Debug Type`)))
  (return _outhits))

(fn `GetTraceParams`
  (returns (StartTraceLocation :type "Vector Structure") (EndTraceLocation :type "Vector Structure") (Orientation :type "Rotator Structure"))
  (bind _half_size_x (`KismetMathLibrary.BreakVector` (`self.Half Size`)))
  (bind (_cameralocation _cameraforwardvector _camerarotation) (`/Game/_Game/Blueprints/Library/BP_GameplayUtilityLibrary.GetCameraTransformInfo` (`self.GetPlayerControllerFromActorInfo`)))
  (bind _returnvalue (+ (`Actor.K2_GetActorLocation` (`self.GetAvatarActorFromActorInfo`)) (* _cameraforwardvector (+ _half_size_x (`self.ExtraOffsetFromPlayer`)))))
  (return _returnvalue (+ _returnvalue (* _cameraforwardvector (`self.TraceLength`))) _camerarotation))

(fn `TargetCanBePushed`
  (params (Hit :type "HitResult Structure (by ref)"))
  (returns (ReturnValue :type Boolean))
  (bind (_bblockinghit _binitialoverlap _time _distance _location _impactpoint _normal _impactnormal _physmat _hitactor) (`GameplayStatics.BreakHitResult` Hit))
  (`/Engine/EditorBlueprintResources/StandardMacros.IsValid` _hitactor
    (:`Is Valid`
      (bind _returnvalue (`/Game/_Game/Blueprints/Library/BP_GameplayLibrary.ActorIsVisible` (`self.GetAvatarActorFromActorInfo`) _hitactor 25.0 true (`self.Draw Debug Type`)))
      (return _returnvalue))
    (:`Is Not Valid`
      (return false))))