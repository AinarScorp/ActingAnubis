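; Gameplay ability that dissolves the avatar's skeletal mesh after death.
; A tick task advances an alpha by delta time and DissolveSpeed, driving the DisolveAmount scalar on the mesh's materials through a lerp.
; On completion it adds the Status.Death.HasDissolved tag to the avatar and ends the ability.
; Activation requires a valid skeletal mesh component in the actor info.
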(event `self.K2_ActivateAbility`
  (set `self.Alpha` 0.0)
  (bind (_asynctaskproxy _deltatime) (`AnubisAbilityTask_TickTask.CreateTickTask` null)
    (:`OnUpdate`
      (set `self.Alpha` (+ (* _deltatime (`self.DissolveSpeed`)) (`self.Alpha`)))
      (`MeshComponent.SetScalarParameterValueOnMaterials` (`.SkeletalMeshComponent` (break `GameplayAbilityActorInfo` (`self.GetActorInfo`))) "DisolveAmount" (`KismetMathLibrary.Lerp` 1.5 -2.0 (`self.Alpha`)))
      (if (>= (`self.Alpha`) 1.0)
        (`AnubisAbilitySystemLibrary.AddStatusTags` (`self.GetAvatarActorFromActorInfo`) (struct :`GameplayTags` (struct :`(TagName` "Status.Death.HasDissolved"))))
        (`self.K2_EndAbility`)))))

(fn `K2_CanActivateAbility`
  (params (ActorInfo :type "GameplayAbilityActorInfo Structure") (Handle :type "GameplayAbilitySpecHandle Structure"))
  (returns (RelevantTags :type "GameplayTagContainer Structure") (ReturnValue :type Boolean))
  (return (struct) (`KismetSystemLibrary.IsValid` (`.SkeletalMeshComponent` (break `GameplayAbilityActorInfo` ActorInfo)))))