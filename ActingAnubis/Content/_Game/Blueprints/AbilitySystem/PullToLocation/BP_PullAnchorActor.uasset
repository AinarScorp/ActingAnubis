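; BP_PullAnchorActor is a placeable anchor for the pull-to-location ability, defining where a pull goes and where it finishes.
; Getter functions convert three offsets (pull, pull finished, line trace check) into world positions rotated by the actor's rotation.
; When the debug flag is set, the construction script flushes persistent debug lines and draws a differently colored, long-lived sphere at each point for editor tuning.
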(fn `DebugPullLocations`
  (if (`self.DebugPullLocation`)
    (`KismetSystemLibrary.FlushPersistentDebugLines`)
    (bind _returnvalue (`self.GetPullLocation`))
    (`KismetSystemLibrary.DrawDebugSphere` _returnvalue 10.0 10 (struct :`R` 1.0 :`B` 0.811978 :`A` 1.0) 99999.0 0.0)
    (bind _returnvalue_2 (`self.GetPullFinishedLocation`))
    (`KismetSystemLibrary.DrawDebugSphere` _returnvalue_2 10.0 10 (struct :`R` 1.0 :`G` 0.934253 :`A` 1.0) 99999.0 0.0)
    (bind _returnvalue_3 (`self.GetLineTraceCheckLocation`))
    (`KismetSystemLibrary.DrawDebugSphere` _returnvalue_3 10.0 10 (struct :`G` 0.253996 :`B` 1.0 :`A` 1.0) 99999.0 0.0)))

(fn `GetLineTraceCheckLocation`
  (returns (ReturnValue :type "Vector Structure"))
  (return (+ (`self.K2_GetActorLocation`) (`KismetMathLibrary.GreaterGreater_VectorRotator` (`self.LineTraceCheckLocationOffset`) (`self.K2_GetActorRotation`)))))

(fn `GetPullFinishedLocation`
  (returns (ReturnValue :type "Vector Structure"))
  (return (+ (`self.K2_GetActorLocation`) (`KismetMathLibrary.GreaterGreater_VectorRotator` (`self.PullFinishedLocationOffset`) (`self.K2_GetActorRotation`)))))

(fn `GetPullLocation`
  (returns (ReturnValue :type "Vector Structure"))
  (return (+ (`self.K2_GetActorLocation`) (`KismetMathLibrary.GreaterGreater_VectorRotator` (`self.PullLocationOffset`) (`self.K2_GetActorRotation`)))))

(fn `UserConstructionScript`
  (`self.DebugPullLocations`))