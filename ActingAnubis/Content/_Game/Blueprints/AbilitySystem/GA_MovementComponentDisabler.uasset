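; Passive gameplay ability that disables and re-enables character movement in response to gameplay events or the MovementComponent.Disabled status tag.
; It activates itself when granted, removing itself if activation fails, and requires a CharacterMovementComponent.
; Chained listener tasks call DisableMovement or restore Walking mode, with a flag ignoring tag removal until setup completes.
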(event `self.BP_OnGiveAbility`
  (params (ActorInfo :type "GameplayAbilityActorInfo Structure (by ref)"))
  (bind ((`AbilitySystemComponent` _abilitysystemcomponent)) (break `GameplayAbilityActorInfo` ActorInfo))
  (bind _returnvalue (`AbilitySystemComponent.TryActivateAbilityByClass` _abilitysystemcomponent "GA_MovementComponentDisabler_C" true))
  (if (not _returnvalue)
    (`/Game/_Game/Blueprints/Library/BP_GameplayLibrary.RemoveAbilitySelf` _abilitysystemcomponent self)))

(event `self.K2_ActivateAbility`
  (`AbilityTask_WaitGameplayEvent.WaitGameplayEvent` (struct :`TagName` "Gameplay.Event.MovementComponent.DisableMovement") null
    (:`then`
      (`AbilityTask_WaitGameplayTagAdded.WaitGameplayTagAdd` (struct :`TagName` "Status.MovementComponent.Disabled") null
        (:`then`
          (`AbilityTask_WaitGameplayTagRemoved.WaitGameplayTagRemove` (struct :`TagName` "Status.MovementComponent.Disabled") null
            (:`then`
              (`AbilityTask_WaitGameplayEvent.WaitGameplayEvent` (struct :`TagName` "Gameplay.Event.MovementComponent.EnableMovement") null
                (:`then`
                  (set `self.bInitializedTasks` true))
                (:`EventReceived`
                  (`self.EnableMovement` :!label _label))))
            (:`Removed`
              (if (`self.bInitializedTasks`)
                (goto _label)))))
        (:`Added`
          (`self.DisableMovement` :!label _label_2))))
    (:`EventReceived`
      (goto _label_2))))

(event `DisableMovement`
  (`CharacterMovementComponent.DisableMovement` (`self.GetCharacterMovementComponent`)))

(event `EnableMovement`
  (`CharacterMovementComponent.SetMovementMode` (`self.GetCharacterMovementComponent`) "MOVE_Walking" 0))

(fn `GetCharacterMovementComponent`
  (returns (`AsCharacter Movement Component` :type "CharacterMovementComponent Object Reference"))
  (bind _ascharacter_movement_component (cast `CharacterMovementComponent` (`.MovementComponent` (break `GameplayAbilityActorInfo` (`self.GetActorInfo`)))))
  (return _ascharacter_movement_component))

(fn `K2_CanActivateAbility`
  (params (ActorInfo :type "GameplayAbilityActorInfo Structure") (Handle :type "GameplayAbilitySpecHandle Structure"))
  (returns (RelevantTags :type "GameplayTagContainer Structure") (ReturnValue :type Boolean))
  (cast `CharacterMovementComponent` (`.MovementComponent` (break `GameplayAbilityActorInfo` ActorInfo))
    (:`then`
      (return (struct) true))
    (:`CastFailed`
      (return (struct) false))))