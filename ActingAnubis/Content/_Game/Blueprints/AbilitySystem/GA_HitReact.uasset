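; Gameplay ability that plays a hit reaction montage and responds only to events with negative magnitude, such as health loss.
; On activation it looks up a montage and section from the owner's gameplay tags plus the health-changed event tag.
; It plays that section and ends on completion, blend out or interruption, or immediately if no animation is found.
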(event `self.K2_ActivateAbility`
  (bind (_bsuccess _animmontage _sectionname) (`/Game/_Game/Blueprints/Library/BP_GameplayLibrary.GetAnimationByIdentifier` (`BlueprintGameplayTagLibrary.GetOwnedGameplayTags` (`self.GetAbilitySystemComponentFromActorInfo`)) (struct :`GameplayTags` (struct :`(TagName` "Gameplay.Event.HealthComponent.Health.Changed")))))
  (if _bsuccess
    (`AbilityTask_PlayMontageAndWait.CreatePlayMontageAndWaitProxy` "None" _animmontage 1.0 _sectionname
      (:`OnCompleted`
        _)
      (:`OnBlendOut`
        _)
      (:`OnInterrupted`
        _))
    (`self.K2_EndAbility`)
    (else
      (`self.K2_EndAbility`))))

(fn `K2_ShouldAbilityRespondToEvent`
  (params (ActorInfo :type "GameplayAbilityActorInfo Structure") (Payload :type "GameplayEventData Structure"))
  (returns (ReturnValue :type Boolean))
  (return (< (`.EventMagnitude` (break `GameplayEventData` Payload)) 0.0)))