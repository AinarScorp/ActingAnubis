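; AI-only gameplay ability that teleports its character to an EQS-chosen location, with a dissolve effect on either side of the jump.
; After the query, it plays a tag-selected montage while a tick task ramps the material's dissolve parameter.
; An Execute gameplay event triggers the move and reverse dissolve, with interruption or a delay as fallback senders.
; A completion event ends the ability; query failure cancels it and sends a failure event.
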(event `SetActorLocationEvent`
  (`Actor.K2_SetActorLocation` (`self.GetAvatarActorFromActorInfo`) (`self.TeleportLocation`) false true)
  (set `self.HasTeleported` true)
  (`self.StartDissolving`))

(event `self.K2_ActivateAbility`
  (bind _returnvalue (`EnvQueryManager.RunEQSQuery` "/Game/_Game/Blueprints/AI/EQS/EQ_FindTeleportLocation.EQ_FindTeleportLocation" (`self.GetAvatarActorFromActorInfo`) "RandomBest25Pct"))
  (add `EnvQueryInstanceBlueprintWrapper.OnQueryFinishedEvent` _returnvalue (delegate `OnQueryFinished`)))

(event `StartAnimationEvent`
  (`AbilityTask_WaitGameplayEvent.WaitGameplayEvent` (struct :`TagName` "Gameplay.Event.Combat.Teleportation.Execute") null true
    (:`then`
      (`self.StartDissolving`)
      (bind (_bsuccess _animmontage _sectionname) (`/Game/_Game/Blueprints/Library/BP_GameplayLibrary.GetAnimationByIdentifier` (`BlueprintGameplayTagLibrary.GetOwnedGameplayTags` (`self.GetAbilitySystemComponentFromActorInfo`)) (struct :`GameplayTags` (struct :`(TagName` "Status.ArtificialIntelligence.Combat.IsTeleporting")))))
      (if _bsuccess
        (`AbilityTask_PlayMontageAndWait.CreatePlayMontageAndWaitProxy` "None" _animmontage 1.0 _sectionname
          (:`then`
            (`self.DebugWithStatusTags` (struct :`GameplayTags` (struct :`(TagName` "Test.Teleport.StartedAnimat")))))
          (:`OnInterrupted`
            (`self.SendGameplayEvent` (struct :`TagName` "Gameplay.Event.Combat.Teleportation.Execute") :!label _label))
          (:`OnCancelled`
            (goto _label)))
        (else
          (`|ExecutionSequence`
            (:`then_0`
              (`KismetSystemLibrary.Delay` 2.0)
              (goto _label))
            (:`then_1`
              (`self.DebugWithStatusTags` (struct :`GameplayTags` (struct :`(TagName` "Test.Teleport.FailedToStartAnim")))))))))
    (:`EventReceived`
      (`self.SetActorLocationEvent`)
      (`self.DebugWithStatusTags` (struct :`GameplayTags` (struct :`(TagName` "Test.Teleport.ReceivedTimingEvent")))))))

(event `OnQueryFinished`
  (params (QueryInstance :type "EnvQueryInstanceBlueprintWrapper Object Reference") (QueryStatus :type "EEnvQueryStatus Enum" :default "Processing"))
  (switch `EEnvQueryStatus` QueryStatus
    (:`Success`
      (bind (_resultlocations _returnvalue) (`EnvQueryInstanceBlueprintWrapper.GetQueryResultsAsLocations` QueryInstance))
      (if _returnvalue
        (set `self.TeleportLocation` (`|GetArrayItem` _resultlocations))
        (`self.DebugWithStatusTags` (struct :`GameplayTags` (struct :`(TagName` "Test.Teleport.TeleportLocationIsSet"))))
        (`self.StartAnimationEvent`)
        (else
          (`KismetSystemLibrary.Delay` 1.0 :!label _label_2)
          (`self.K2_CancelAbility`)
          (`self.SendGameplayEvent` (struct :`TagName` "Gameplay.Event.Combat.Teleportation.TeleportedToBetterPosition.Failed")))))
    (:`Failed`
      (goto _label_2))))

(event `StartDissolving`
  (bind _alpha (`self.Alpha`))
  (`self.DebugWithStatusTags` (select `bool` (`self.HasTeleported`) :`false` (struct :`GameplayTags` (struct :`(TagName` "Test.Teleport.DissolvingBeforeTeleport"))) :`true` (struct :`GameplayTags` (struct :`(TagName` "Test.Teleport.DissolvingAfterTeleport"))) :!type "GameplayTagContainer Structure"))
  (bind (_asynctaskproxy _deltatime) (`AnubisAbilityTask_TickTask.CreateTickTask` null)
    (:`then`
      (set `self.DissolveTask` _asynctaskproxy))
    (:`OnUpdate`
      (set `self.Alpha` (+ (`self.Alpha`) (* (* _deltatime (`self.DissolveSpeed`)) (`KismetMathLibrary.SelectFloat` -1.0 1.0 (`self.HasTeleported`)))))
      (`self.SetDissolveParam`)
      (if (select `bool` (`self.HasTeleported`) :`false` (>= _alpha 1.0) :`true` (<= _alpha 0.0))
        (`|ExecutionSequence`
          (:`then_0`
            (if (`self.HasTeleported`)
              (`self.SendGameplayEvent` (struct :`TagName` "Gameplay.Event.Combat.Teleportation.TeleportedToBetterPosition"))
              (`self.K2_EndAbility`)
              (else
                (`GameplayTask.EndTask` (`self.DissolveTask`))))))))))

(event `self.K2_OnEndAbility`
  (params (bWasCancelled :type Boolean))
  (`|ExecutionSequence`
    (:`then_0`
      (set `self.HasTeleported` false)
      (set `self.Alpha` 0.0)
      (set `self.DissolveTask` null))
    (:`then_1`
      (if bWasCancelled
        (`self.SetDissolveParam`)))
    (:`then_2`
      (if (not bWasCancelled)
        (`AbilitySystemBlueprintLibrary.RemoveLooseGameplayTags` (`self.GetAvatarActorFromActorInfo`) (`BlueprintGameplayTagLibrary.MakeLiteralGameplayTagContainer` (struct :`GameplayTags` (struct :`(TagName` "Test.Teleport.TeleportLocationIsSet") :`(TagName` "Test.Teleport.StartedAnimat") :`(TagName` "Test.Teleport.FailedToStartAnim") :`(TagName` "Test.Teleport.ReceivedTimingEvent") :`(TagName` "Test.Teleport.DissolvingBeforeTeleport") :`(TagName` "Test.Teleport.DissolvingAfterTeleport")))))))))

(fn `DebugWithStatusTags`
  (params (Value :type "GameplayTagContainer Structure"))
  (`AnubisAbilitySystemLibrary.AddStatusTags` (`self.GetAvatarActorFromActorInfo`) (`BlueprintGameplayTagLibrary.MakeLiteralGameplayTagContainer` Value)))

(fn `K2_CanActivateAbility`
  (params (ActorInfo :type "GameplayAbilityActorInfo Structure") (Handle :type "GameplayAbilitySpecHandle Structure"))
  (returns (RelevantTags :type "GameplayTagContainer Structure") (ReturnValue :type Boolean))
  (return (struct) (`KismetSystemLibrary.IsValid` (`AIBlueprintHelperLibrary.GetAIController` ActorInfo_AvatarActor))))

(fn `SetDissolveParam`
  (`MeshComponent.SetScalarParameterValueOnMaterials` (`.SkeletalMeshComponent` (break `GameplayAbilityActorInfo` (`self.GetActorInfo`))) "DisolveAmount" (`KismetMathLibrary.Lerp` 1.5 -2.0 (`self.Alpha`))))