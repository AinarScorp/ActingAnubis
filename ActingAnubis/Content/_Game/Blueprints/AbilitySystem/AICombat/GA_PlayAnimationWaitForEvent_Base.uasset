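; Base AI combat gameplay ability that plays an animation and waits for a gameplay event to trigger its effect.
; Activation requires an identifier tag and looks up a montage using owned tags, extra tags and the awaited event tag.
; The event calls the empty OnReceivedWaitingEvent hook and ends the ability, as does montage completion, interruption or cancellation.
; Without a matching animation, it sends the event itself after a short delay.
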(event `self.K2_ActivateAbilityFromEvent`
  (params (EventData :type "GameplayEventData Structure (by ref)"))
  (bind _alltagstosend (`self.AllTagsToSend`))
  (`AbilityTask_WaitGameplayEvent.WaitGameplayEvent` (`self.EventToWaitForForExecution`) null true
    (:`then`
      (bind _tagcontainer (`AnubisAbilitySystemLibrary.GetOwnedGameplayTags` (`self.GetAvatarActorFromActorInfo`)))
      (set `self.AllTagsToSend` _tagcontainer)
      (`BlueprintGameplayTagLibrary.AppendGameplayTagContainers` _alltagstosend (`self.Extra Tags Params For Finding Animations`))
      (`BlueprintGameplayTagLibrary.AddGameplayTag` _alltagstosend (`self.EventToWaitForForExecution`))
      (bind (_bsuccess _animmontage _sectionname) (`/Game/_Game/Blueprints/Library/BP_GameplayLibrary.GetAnimationByIdentifier` _alltagstosend))
      (if _bsuccess
        (`AbilityTask_PlayMontageAndWait.CreatePlayMontageAndWaitProxy` "None" _animmontage 1.0 _sectionname
          (:`OnCompleted`
            _)
          (:`OnInterrupted`
            _)
          (:`OnCancelled`
            _))
        (`self.K2_EndAbility`)
        (else
          (`KismetSystemLibrary.Delay` 3.0)
          (`self.SendGameplayEvent` (`self.EventToWaitForForExecution`)))))
    (:`EventReceived`
      (`self.OnReceivedWaitingEvent`)
      (`self.K2_EndAbility`))))

(fn `K2_CanActivateAbility`
  (params (ActorInfo :type "GameplayAbilityActorInfo Structure") (Handle :type "GameplayAbilitySpecHandle Structure"))
  (returns (RelevantTags :type "GameplayTagContainer Structure") (ReturnValue :type Boolean))
  (bind _bsuccess (`/Game/_Game/Blueprints/Library/BP_GameplayLibrary.GetIdentifierTag` (`BlueprintGameplayTagLibrary.GetOwnedGameplayTags` (`.AbilitySystemComponent` (break `GameplayAbilityActorInfo` ActorInfo)))))
  (return (struct) _bsuccess))

(fn `OnReceivedWaitingEvent`)