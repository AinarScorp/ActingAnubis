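; Gameplay ability that randomly prompts flying AI creatures to switch between flying and walking.
; It activates itself when granted and starts a timer with a random delay, apparently driving a percentage-chance roll.
; On success it adds a ShouldChangeState status tag, waits for the opposite movement-mode tag, then removes the request and restarts the timer.
; A failed roll simply restarts the timer.
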(event `self.K2_ActivateAbility`
  (`self.StartTimer`))

(event `TryChangeTimer`
  (bind _returnvalue (`self.GetAvatarActorFromActorInfo`))
  (if (<= (`KismetMathLibrary.RandomFloatInRange` 0.0 100.0) (`self.ChancePercent`))
    (`AnubisAbilitySystemLibrary.AddStatusTags` _returnvalue (struct :`GameplayTags` (struct :`(TagName` "Status.FlyingCreatures.ShouldChangeState"))))
    (bind _returnvalue_2 (`AnubisAbilitySystemLibrary.HasMatchingGameplayTag` _returnvalue (struct :`TagName` "Status.MovementMode.Flying")))
    (`AbilityTask_WaitGameplayTagAdded.WaitGameplayTagAdd` (select `bool` _returnvalue_2 :`false` (struct :`TagName` "Status.MovementMode.Flying") :`true` (struct :`TagName` "Status.MovementMode.Walking") :!type "GameplayTag Structure") null true
      (:`Added`
        (`AnubisAbilitySystemLibrary.RemoveStatusTags` (`self.GetAvatarActorFromActorInfo`) (struct :`GameplayTags` (struct :`(TagName` "Status.FlyingCreatures.ShouldChangeState"))))
        (`self.StartTimer`)))
    (else
      (`self.StartTimer`))))

(event `self.BP_OnGiveAbility`
  (params (ActorInfo :type "GameplayAbilityActorInfo Structure (by ref)"))
  (`AbilitySystemComponent.TryActivateAbilityByClass` (`.AbilitySystemComponent` (break `GameplayAbilityActorInfo` ActorInfo)) "GA_ChangeFlyingState_C" true))

(fn `StartTimer`
  (`KismetSystemLibrary.K2_SetTimerDelegate` (`|CreateDelegate` :!event `TryChangeTimer`) (`KismetMathLibrary.RandomFloatInRange` (`self.MinTimer`) (`self.MaxTimer`))))