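; GA_Shoot is an AI combat gameplay ability that fires a BP_Projectile at the player.
; OnReceivedWaitingEvent triggers the spawn, with the avatar as owner and rotation aimed from the avatar's location, not the muzzle, toward player pawn 0.
; The spawn point is the ShootProjectileSpawnLocation socket, marked by a debug sphere.
; Without it, a rotated offset from the avatar is used, with an on-screen warning if a skeletal mesh lacks the socket.
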(fn `GetProjectileSpawnLocation`
  (returns (ReturnValue :type "Vector Structure"))
  (bind ((`SkeletalMeshComponent` _skeletalmeshcomponent)) (break `GameplayAbilityActorInfo` (`self.GetActorInfo`)))
  (bind (_returnvalue_location _returnvalue_rotation) (`KismetMathLibrary.BreakTransform` (`Actor.GetTransform` (`self.GetAvatarActorFromActorInfo`))))
  (bind _returnvalue (`SceneComponent.GetSocketLocation` _skeletalmeshcomponent "ShootProjectileSpawnLocation"))
  (`|ExecutionSequence`
    (:`then_0`
      (`/Engine/EditorBlueprintResources/StandardMacros.IsValid` _skeletalmeshcomponent
        (:`Is Valid`
          (if (`SceneComponent.DoesSocketExist` _skeletalmeshcomponent "ShootProjectileSpawnLocation")
            (`KismetSystemLibrary.DrawDebugSphere` _returnvalue 24.0 12 (struct :`R` 1.0 :`G` 1.0 :`B` 1.0 :`A` 1.0) 30.0)
            (return _returnvalue)
            (else
              (`KismetSystemLibrary.PrintText` (`|FormatText` "Projectile has been shot from an actor with a skeltal Mesh. \nNo Socket With a name  {Name} Has been found. \nPlease Add that socket on {Skeleton Name} then projectile will shoot from there" (`self.SocketName`) (`KismetSystemLibrary.GetDisplayName` _skeletalmeshcomponent)) true true (struct :`R` 1.0 :`A` 1.0) 30.0))))))
    (:`then_1`
      (return (+ _returnvalue_location (`KismetMathLibrary.GreaterGreater_VectorRotator` (`self.SpawnProjectileOffset`) _returnvalue_rotation))))))

(fn `OnReceivedWaitingEvent`
  (`self.SpawnProjectile`))

(fn `SpawnProjectile`
  (bind _returnvalue (`self.GetAvatarActorFromActorInfo`))
  (bind (_returnvalue_location _returnvalue_rotation) (`KismetMathLibrary.BreakTransform` (`Actor.GetTransform` _returnvalue)))
  (`|SpawnActorFromClass` "/Game/_Game/Blueprints/Enemies/BP_Projectile.BP_Projectile_C" (`KismetMathLibrary.MakeTransform` (`self.GetProjectileSpawnLocation`) (`KismetMathLibrary.Conv_VectorToRotator` (`KismetMathLibrary.GetDirectionUnitVector` _returnvalue_location (`Actor.K2_GetActorLocation` (`GameplayStatics.GetPlayerPawn` 0))))) "AlwaysSpawn" "MultiplyWithRoot" _returnvalue null))