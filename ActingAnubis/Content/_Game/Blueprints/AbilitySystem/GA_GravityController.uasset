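; Passive gameplay ability that switches its owner's CharacterMovementComponent gravity off and back on.
; It activates when granted, removes itself if activation fails, and requires a CharacterMovementComponent.
; Disable/Enable gameplay events or adding/removing the Gravity.Disabled tag cache and zero GravityScale, or restore it.
; An initialization flag ignores tag removal during task setup, and restoring resets the cache to the activation-time default.
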(event `self.BP_OnGiveAbility`
  (params (ActorInfo :type "GameplayAbilityActorInfo Structure (by ref)"))
  (bind ((`AbilitySystemComponent` _abilitysystemcomponent)) (break `GameplayAbilityActorInfo` ActorInfo))
  (bind _returnvalue (`AbilitySystemComponent.TryActivateAbilityByClass` _abilitysystemcomponent "GA_GravityController_C" true))
  (if (not _returnvalue)
    (`/Game/_Game/Blueprints/Library/BP_GameplayLibrary.RemoveAbilitySelf` _abilitysystemcomponent self)))

(event `self.K2_ActivateAbility`
  (`self.CacheGravityScale`)
  (set `self.DefaultGravityScale` (`self.CachedGravityScale`))
  (`AbilityTask_WaitGameplayEvent.WaitGameplayEvent` (struct :`TagName` "Gameplay.Event.MovementComponent.Gravity.Disable") null
    (:`then`
      (`AbilityTask_WaitGameplayTagAdded.WaitGameplayTagAdd` (struct :`TagName` "Status.MovementComponent.Gravity.Disabled") null
        (:`then`
          (`AbilityTask_WaitGameplayTagRemoved.WaitGameplayTagRemove` (struct :`TagName` "Status.MovementComponent.Gravity.Disabled") null
            (:`then`
              (`AbilityTask_WaitGameplayEvent.WaitGameplayEvent` (struct :`TagName` "Gameplay.Event.MovementComponent.Gravity.Enable") null
                (:`then`
                  (set `self.bInitializedTasks` true))
                (:`EventReceived`
                  (`self.RestoreGravityScale` :!label _label))))
            (:`Removed`
              (if (`self.bInitializedTasks`)
                (goto _label)))))
        (:`Added`
          (bind _character_movement_component (`self.CacheGravityScale` :!label _label_2))
          (set `CharacterMovementComponent.GravityScale` 0.0 _character_movement_component))))
    (:`EventReceived`
      (goto _label_2))))

(fn `CacheGravityScale`
  (returns (`Character Movement Component` :type "CharacterMovementComponent Object Reference"))
  (locals (CMC :type "CharacterMovementComponent Object Reference"))
  (bind _output_get (set `local.CMC` (`self.GetCharacterMovementComponent`)))
  (set `self.CachedGravityScale` (`CharacterMovementComponent.GravityScale` _output_get))
  (return _output_get))

(fn `GetCharacterMovementComponent`
  (returns (`AsCharacter Movement Component` :type "CharacterMovementComponent Object Reference"))
  (bind _ascharacter_movement_component (cast `CharacterMovementComponent` (`.MovementComponent` (break `GameplayAbilityActorInfo` (`self.GetActorInfo`)))))
  (return _ascharacter_movement_component))

(fn `K2_CanActivateAbility`
  (params (ActorInfo :type "GameplayAbilityActorInfo Structure") (Handle :type "GameplayAbilitySpecHandle Structure"))
  (returns (RelevantTags :type "GameplayTagContainer Structure") (ReturnValue :type Boolean))
  (cast `CharacterMovementComponent` (`.MovementComponent` (break `GameplayAbilityActorInfo` ActorInfo))
    (:`then`
      (return (struct) true))
    (:`CastFailed`
      (return (struct) false))))

(fn `RestoreGravityScale`
  (set `CharacterMovementComponent.GravityScale` (`self.CachedGravityScale`) (`self.GetCharacterMovementComponent`))
  (set `self.CachedGravityScale` (`self.DefaultGravityScale`)))