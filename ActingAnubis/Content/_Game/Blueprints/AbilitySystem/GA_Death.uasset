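; GA_Death is an event-activated gameplay ability that runs the avatar's dying sequence.
; It calls CancelAllAbilities with the Death tag, then starts dying on BP_HealthComponent.
; It looks up a montage by the owner's gameplay tags and, if found, plays it without stopping when the ability ends.
; Independently of the montage, a DyingStateTimer delay leads to FinishDying and ends the ability.
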(event `self.K2_ActivateAbilityFromEvent`
  (params (EventData :type "GameplayEventData Structure (by ref)"))
  (bind _returnvalue (`Actor.GetComponentByClass` (`self.GetAvatarActorFromActorInfo`) "/Game/_Game/Blueprints/BP_HealthComponent.BP_HealthComponent_C"))
  (`self.BP_CancelAllAbilities` (struct :`GameplayTags` (struct :`(TagName` "Gameplay.Ability.Death"))))
  (`/Game/_Game/Blueprints/BP_HealthComponent.StartDying` _returnvalue)
  (bind (_bsuccess _animmontage _sectionname) (`/Game/_Game/Blueprints/Library/BP_GameplayLibrary.GetAnimationByIdentifier` (`BlueprintGameplayTagLibrary.GetOwnedGameplayTags` (`self.GetAbilitySystemComponentFromActorInfo`))))
  (`|ExecutionSequence`
    (:`then_0`
      (if _bsuccess
        (`AbilityTask_PlayMontageAndWait.CreatePlayMontageAndWaitProxy` "None" _animmontage 1.0 _sectionname false)))
    (:`then_1`
      (`KismetSystemLibrary.Delay` (`self.DyingStateTimer`))
      (`/Game/_Game/Blueprints/BP_HealthComponent.FinishDying` _returnvalue false)
      (`self.K2_EndAbility`))))