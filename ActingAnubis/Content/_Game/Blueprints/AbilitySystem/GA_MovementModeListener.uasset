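; Passive gameplay ability that mirrors a Character's movement mode as Status.MovementMode gameplay tags on the avatar.
; It tries to activate itself when granted, requires a Character avatar, and removes itself if activation fails.
; On activation it adds the current mode's tag and binds to the movement-mode-changed delegate, swapping old and new tags on each change.
; Ending the ability unbinds the delegate.
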(event `self.BP_OnGiveAbility`
  (params (ActorInfo :type "GameplayAbilityActorInfo Structure (by ref)"))
  (bind (_owneractor _avataractor _playercontroller _abilitysystemcomponent) (break `GameplayAbilityActorInfo` ActorInfo))
  (bind _returnvalue (`AbilitySystemComponent.TryActivateAbilityByClass` _abilitysystemcomponent "GA_MovementModeListener_C" true))
  (if (not _returnvalue)
    (`/Game/_Game/Blueprints/Library/BP_GameplayLibrary.RemoveAbilitySelf` _abilitysystemcomponent self)))

(event `self.K2_ActivateAbility`
  (`self.AddCurrentMovementModeStatus` (`self.GetCharacterMovementComponent`))
  (bind _ascharacter (cast `Character` (`self.GetAvatarActorFromActorInfo`)))
  (add `Character.MovementModeChangedDelegate` _ascharacter (`|CreateDelegate` :!event `UpdateMovementModeStatus`)))

(event `UpdateMovementModeStatus`
  (params (Character :type "Character Object Reference") (PrevMovementMode :type "EMovementMode Enum" :default "MOVE_None") (PreviousCustomMode :type Byte))
  (bind _charactermovement (`Character.CharacterMovement` Character))
  (if (not (`|EnumEquality` (`CharacterMovementComponent.MovementMode` _charactermovement) PrevMovementMode))
    (`self.RemoveMovementModeStatus` PrevMovementMode)
    (`self.AddCurrentMovementModeStatus` _charactermovement)))

(event `self.K2_OnEndAbility`
  (params (bWasCancelled :type Boolean))
  (bind _ascharacter (cast `Character` (`self.GetAvatarActorFromActorInfo`)))
  (remove `Character.MovementModeChangedDelegate` _ascharacter (`|CreateDelegate` :!event `UpdateMovementModeStatus`)))

(fn `AddCurrentMovementModeStatus`
  (params (CharacterMovementComponent :type "CharacterMovementComponent Object Reference"))
  (`AnubisAbilitySystemLibrary.AddStatusTags` (`self.GetAvatarActorFromActorInfo`) (`BlueprintGameplayTagLibrary.MakeGameplayTagContainerFromTag` (`self.GetTagFromMovementMode` (`CharacterMovementComponent.MovementMode` CharacterMovementComponent)))))

(fn `GetCharacterMovementComponent`
  (returns (ReturnValue :type "CharacterMovementComponent Object Reference"))
  (bind _ascharacter_movement_component (cast `CharacterMovementComponent` (`.MovementComponent` (break `GameplayAbilityActorInfo` (`self.GetActorInfo`)))))
  (return _ascharacter_movement_component))

(fn `GetTagFromMovementMode`
  (params (MovementMode :type "EMovementMode Enum" :default "MOVE_None"))
  (returns (ReturnValue :type "GameplayTag Structure"))
  (return (select `EMovementMode` MovementMode :`MOVE_None` (struct :`TagName` "Status.MovementMode.None") :`MOVE_Walking` (struct :`TagName` "Status.MovementMode.Walking") :`MOVE_NavWalking` (struct :`TagName` "Status.MovementMode.NavmeshWalking") :`MOVE_Falling` (struct :`TagName` "Status.MovementMode.Falling") :`MOVE_Swimming` (struct :`TagName` "Status.MovementMode.Swimming") :`MOVE_Flying` (struct :`TagName` "Status.MovementMode.Flying") :`MOVE_Custom` (struct :`TagName` "Status.MovementMode.Custom") :!type "GameplayTag Structure")))

(fn `K2_CanActivateAbility`
  (params (ActorInfo :type "GameplayAbilityActorInfo Structure") (Handle :type "GameplayAbilitySpecHandle Structure"))
  (returns (RelevantTags :type "GameplayTagContainer Structure") (ReturnValue :type Boolean))
  (cast `Character` (`.AvatarActor` (break `GameplayAbilityActorInfo` ActorInfo))
    (:`then`
      (return (struct) true))
    (:`CastFailed`
      (return (struct) false))))

(fn `RemoveMovementModeStatus`
  (params (OldMovementMode :type "EMovementMode Enum" :default "MOVE_None"))
  (`AnubisAbilitySystemLibrary.RemoveStatusTags` (`self.GetAvatarActorFromActorInfo`) (`BlueprintGameplayTagLibrary.MakeGameplayTagContainerFromTag` (`self.GetTagFromMovementMode` OldMovementMode))))