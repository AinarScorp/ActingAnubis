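; GA_Shoot is a gameplay ability that fires a single BP_Projectile from its avatar toward the first player's pawn, and activates only if an identifier tag is found among owned tags.
; It listens for the Shoot.Execute gameplay event to spawn the projectile, while playing a montage chosen from the avatar's tags.
; Without a matching montage, it sends that event itself and ends after a short delay; otherwise it ends with the montage.
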(event `self.K2_ActivateAbilityFromEvent`
  (params (EventData :type "GameplayEventData Structure (by ref)"))
  (bind _returnvalue (`self.GetAvatarActorFromActorInfo`))
  (bind (_returnvalue_location _returnvalue_rotation) (`KismetMathLibrary.BreakTransform` (`Actor.GetTransform` _returnvalue)))
  (`AbilityTask_WaitGameplayEvent.WaitGameplayEvent` (struct :`TagName` "Gameplay.Event.Combat.Shoot.Execute") null true
    (:`then`
      (bind _tagcontainer (`AnubisAbilitySystemLibrary.GetOwnedGameplayTags` (`self.GetAvatarActorFromActorInfo`)))
      (bind (_bsuccess _animmontage _sectionname) (`/Game/_Game/Blueprints/Library/BP_GameplayLibrary.GetAnimationByIdentifier` _tagcontainer (struct :`GameplayTags` (struct :`(TagName` "Gameplay.Event.Combat.Shoot")))))
      (if _bsuccess
        (`AbilityTask_PlayMontageAndWait.CreatePlayMontageAndWaitProxy` "None" _animmontage 1.0 _sectionname
          (:`OnCompleted`
            _)
          (:`OnInterrupted`
            _)
          (:`OnCancelled`
            _))
        (`self.K2_EndAbility`)
        (else
          (`self.SendGameplayEvent` (struct :`TagName` "Gameplay.Event.Combat.Shoot.Execute"))
          (`KismetSystemLibrary.Delay` 2.0)
          (`self.K2_EndAbility`))))
    (:`EventReceived`
      (`|SpawnActorFromClass` "/Game/DominikTestStuff/Blueprints/BP_Projectile.BP_Projectile_C" (`KismetMathLibrary.MakeTransform` (+ _returnvalue_location (`KismetMathLibrary.GreaterGreater_VectorRotator` (`self.SpawnLocationOffset`) _returnvalue_rotation)) (`KismetMathLibrary.Conv_VectorToRotator` (`KismetMathLibrary.GetDirectionUnitVector` _returnvalue_location (`Actor.K2_GetActorLocation` (`GameplayStatics.GetPlayerPawn` 0))))) "AdjustIfPossibleButAlwaysSpawn" "MultiplyWithRoot" _returnvalue null))))

(fn `K2_CanActivateAbility`
  (params (ActorInfo :type "GameplayAbilityActorInfo Structure") (Handle :type "GameplayAbilitySpecHandle Structure"))
  (returns (RelevantTags :type "GameplayTagContainer Structure") (ReturnValue :type Boolean))
  (bind _bsuccess (`/Game/_Game/Blueprints/Library/BP_GameplayLibrary.GetIdentifierTag` (`BlueprintGameplayTagLibrary.GetOwnedGameplayTags` (`.AbilitySystemComponent` (break `GameplayAbilityActorInfo` ActorInfo)))))
  (return (struct) _bsuccess))