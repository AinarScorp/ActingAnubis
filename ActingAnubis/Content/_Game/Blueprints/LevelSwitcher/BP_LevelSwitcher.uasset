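; BP_LevelSwitcher is an actor that moves the player through a sequence of levels by teleporting between player starts.
; Its PlayerStarts array pairs each level's start point with a portal.
; LevelComplete records the finished level's index and activates that level's portal.
; OnPortalEntered teleports player 0's character to the next start's location and rotation, doing nothing after the last entry.
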(fn `LevelComplete`
  (params (LevelIndex :type Integer))
  (set `self.CurrentLevelIndex` LevelIndex)
  (`/Game/DominikTestStuff/Blueprints/BP_Portal.ActivatePortal` (`.Portal_5_D9AD02E24E17B6E1569F06A6B5AB7B57` (break `/Game/_Game/Blueprints/LevelSwitcher/S_LevelSwitcherInfo` (`|GetArrayItem` (`self.PlayerStarts`) (`self.CurrentLevelIndex`))))))

(fn `OnPortalEntered`
  (bind _playerstarts (`self.PlayerStarts`))
  (bind _output_playerstart (break `/Game/_Game/Blueprints/LevelSwitcher/S_LevelSwitcherInfo` (`|GetArrayItem` _playerstarts (+ (`self.CurrentLevelIndex`) 1))))
  (bind (_returnvalue_location _returnvalue_rotation) (`KismetMathLibrary.BreakTransform` (`self.GetTransform` _output_playerstart)))
  (if (< (+ (`self.CurrentLevelIndex`) 1) (`KismetArrayLibrary.Array_Length` _playerstarts))
    (`self.K2_SetActorLocationAndRotation` (`GameplayStatics.GetPlayerCharacter` 0) _returnvalue_location _returnvalue_rotation false true)))

(fn `UserConstructionScript`)