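; Level-switcher Blueprint that completes the level once every enemy in its EnemiesToKeepTrackOn list has died.
; On BeginPlay it waits once on each listed enemy for the HealthComponent OutOfHealth gameplay event and counts the deaths, printing a debug message for each.
; When the count matches the list length, it calls LevelComplete on AnubisGameMode with its LevelIndex.
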(event `self.ReceiveBeginPlay`
  (for _array_element (`self.EnemiesToKeepTrackOn`)
    (`AbilityAsync_WaitGameplayEvent.WaitGameplayEventToActor` _array_element (struct :`TagName` "Gameplay.Event.HealthComponent.Death.OutOfHealth") true
      (:`EventReceived`
        (`/Engine/EditorBlueprintResources/StandardMacros.IncrementInt` (`self.DeadEnemyCount`)
          (:`  `
            (`KismetSystemLibrary.PrintString` "ENEMY DIED" true true (struct :`R` 1.0 :`G` 0.16148 :`A` 1.0) 800000.0)
            (if (== (`self.DeadEnemyCount`) (`KismetArrayLibrary.Array_Length` (`self.EnemiesToKeepTrackOn`)))
              (bind _asanubis_game_mode (cast `/Game/DominikTestStuff/Levels/Game/AnubisGameMode` (`GameplayStatics.GetGameMode`)))
              (`/Game/DominikTestStuff/Levels/Game/AnubisGameMode.LevelComplete` _asanubis_game_mode (`self.Level Index`)))))))))

(fn `UserConstructionScript`)