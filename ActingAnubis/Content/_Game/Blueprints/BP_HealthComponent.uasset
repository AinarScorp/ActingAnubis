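; Health component that tracks an actor's current and max health, driven by gameplay events.
; On BeginPlay it loads starting values from DT_StartingHealth, using an override tag or the owner's Identifier tag as row name.
; Damage, healing and max-health events sent to the owner update clamped values, which broadcast change events, plus OutOfHealth at zero.
; Separate StartDying and FinishDying functions manage Dying and Dead status tags and call matching events.
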(event `self.ReceiveBeginPlay`
  (bind _returnvalue (`self.GetOwner`))
  (`self.RegisterHealth`)
  (bind (_asynctaskproxy _payload) (`AbilityAsync_WaitGameplayEvent.WaitGameplayEventToActor` _returnvalue (struct :`TagName` "Gameplay.Event.HealthComponent.Damage"))
    (:`then`
      (bind (_asynctaskproxy_2 _payload_2) (`AbilityAsync_WaitGameplayEvent.WaitGameplayEventToActor` _returnvalue (struct :`TagName` "Gameplay.Event.HealthComponent.Healing"))
        (:`then`
          (bind (_asynctaskproxy_3 _payload_3) (`AbilityAsync_WaitGameplayEvent.WaitGameplayEventToActor` _returnvalue (struct :`TagName` "Gameplay.Event.HealthComponent.MaxHealth.Modify"))
            (:`EventReceived`
              (bind ((`Instigator` _instigator) (`EventMagnitude` _eventmagnitude)) (break `GameplayEventData` _payload_3))
              (`self.ModifyMaxHealth` _instigator _eventmagnitude))))
        (:`EventReceived`
          (`self.HealHealth` _payload_2))))
    (:`EventReceived`
      (`self.DamageHealth` _payload))))

(fn `CheckIfMultipleIdentifiers`
  (params (AllTags :type "Array of GameplayTag Structure") (ChosenTag :type Name))
  (if (> (`KismetArrayLibrary.Array_Length` AllTags) 1)
    (`KismetSystemLibrary.PrintText` (`|FormatText` "{Owner Name} Has Multiple Identifiers, Only first one will be used : {tag}, If you need multiple Identifiers Override the available tag for this component" (`KismetSystemLibrary.GetDisplayName` (`self.GetOwner`)) ChosenTag) true true (struct :`R` 1.0 :`A` 1.0) 10.0)))

(fn `DamageHealth`
  (params (GameplayEventData :type "GameplayEventData Structure (by ref)"))
  (bind ((`Instigator` _instigator) (`EventMagnitude` _eventmagnitude)) (break `GameplayEventData` GameplayEventData))
  (`self.ModifyHealth` _instigator (* (`KismetMathLibrary.Abs` _eventmagnitude) -1.0)))

(fn `FinishDying`
  (params (IgnoredStartDying :type Boolean))
  (bind _returnvalue (`self.GetOwner`))
  (`|ExecutionSequence`
    (:`then_0`
      (if (not IgnoredStartDying)
        (`AnubisAbilitySystemLibrary.RemoveStatusTags` _returnvalue (struct :`GameplayTags` (struct :`(TagName` "Status.HealthComponent.IsDying"))))))
    (:`then_1`
      (`AnubisAbilitySystemLibrary.AddStatusTags` _returnvalue (struct :`GameplayTags` (struct :`(TagName` "Status.HealthComponent.Dead")))))
    (:`then_2`
      (`self.FinishDyingEvent`))))

(fn `GetHealth`
  (returns (CurrentHealth :type "Float (double-precision)"))
  (return (`self.CurrentHealth`)))

(fn `GetHealthStats`
  (returns (CurrentHealth :type "Float (double-precision)") (MaxHealth :type "Float (double-precision)"))
  (return (`self.CurrentHealth`) (`self.MaxHealth`)))

(fn `GetMaxHealth`
  (returns (MaxHealth :type "Float (double-precision)"))
  (return (`self.MaxHealth`)))

(fn `HealHealth`
  (params (GameplayEventData :type "GameplayEventData Structure (by ref)"))
  (bind ((`Instigator` _instigator) (`EventMagnitude` _eventmagnitude)) (break `GameplayEventData` GameplayEventData))
  (`self.ModifyHealth` _instigator (`KismetMathLibrary.Abs` _eventmagnitude)))

(fn `ModifyHealth`
  (params (Instigator :type "Actor Object Reference") (DeltaMaxHealth :type "Float (double-precision)"))
  (locals (NewHealth :type "Float (double-precision)"))
  (bind ((`GameplayEventData` _gameplayeventdata)) (make `GameplayEventData` :`Instigator` (`local.Instigator`) :`EventMagnitude` DeltaMaxHealth))
  (bind _output_get (set `local.NewHealth` (+ DeltaMaxHealth (`self.CurrentHealth`))))
  (set `self.CurrentHealth` (`KismetMathLibrary.FClamp` _output_get 0.0 (`self.MaxHealth`)))
  (`AbilitySystemBlueprintLibrary.SendGameplayEventToActor` (`self.GetOwner`) (struct :`TagName` "Gameplay.Event.HealthComponent.Health.Changed") _gameplayeventdata)
  (if (<= (`self.CurrentHealth`) 0.0)
    (`AbilitySystemBlueprintLibrary.SendGameplayEventToActor` (`self.GetOwner`) (struct :`TagName` "Gameplay.Event.HealthComponent.Death.OutOfHealth") _gameplayeventdata)))

(fn `ModifyMaxHealth`
  (params (Instigator :type "Actor Object Reference") (DeltaMaxHealth :type "Float (double-precision)"))
  (locals (NewMaxHealth :type "Float (double-precision)"))
  (bind _output_get (set `local.NewMaxHealth` (+ DeltaMaxHealth (`self.MaxHealth`))))
  (set `self.MaxHealth` (`KismetMathLibrary.FClamp` _output_get 1.0 999999999.0))
  (`AbilitySystemBlueprintLibrary.SendGameplayEventToActor` (`self.GetOwner`) (struct :`TagName` "Gameplay.Event.HealthComponent.MaxHealth.Changed") (make `GameplayEventData` :`Instigator` (`local.Instigator`) :`EventMagnitude` (`self.MaxHealth`))))

(fn `RegisterHealth`
  (locals (ChosenTag :type Name :default "None"))
  (bind _overrideidentifier (`self.OverrideIdentifier`))
  (`|ExecutionSequence`
    (:`then_0`
      (if (`BlueprintGameplayTagLibrary.IsGameplayTagValid` _overrideidentifier)
        (set `local.ChosenTag` (`BlueprintGameplayTagLibrary.GetTagName` _overrideidentifier))
        (else
          (bind _tagcontainer (`AnubisAbilitySystemLibrary.GetOwnedGameplayTags` (`self.GetOwner`)))
          (bind _returnvalue (`AnubisAbilitySystemLibrary.FilterTagContainer` _tagcontainer (`BlueprintGameplayTagLibrary.MakeGameplayTagContainerFromTag` (struct :`TagName` "Identifier"))))
          (bind _gameplaytags (`BlueprintGameplayTagLibrary.BreakGameplayTagContainer` _returnvalue))
          (if (`KismetArrayLibrary.Array_IsEmpty` _gameplaytags)
            (`KismetSystemLibrary.PrintText` (`|FormatText` "{OwnerName} Was Unable To Init StartingHealth, No Identifier has been found, make sure that this actor has Either Identifier. Tag on him, or OverrideIdentifier is Not Empty \nFound Identifier{ID} " (`KismetSystemLibrary.GetDisplayName` (`self.GetOwner`)) (`local.ChosenTag`)) true true (struct :`R` 1.0 :`A` 1.0) 99.0)
            (return)
            (else
              (bind _output_get (set `local.ChosenTag` (`BlueprintGameplayTagLibrary.GetTagName` (`|GetArrayItem` _gameplaytags))))
              (`self.CheckIfMultipleIdentifiers` _gameplaytags _output_get))))))
    (:`then_1`
      (bind _returnvalue_2 (`|GetDataTableRow` "/Game/_Game/Health_And_Damage/DT_StartingHealth.DT_StartingHealth" (`local.ChosenTag`))
        (:`then`
          (bind ((`StartingMaxHealth_4_C0E3B68F4984F16124D15F899C72E486` _startingmaxhealth) (`StartingHealthIsDifferentFromMaxHealth_10_ADF20C114763E6CBE25D65B9A03A9171` _startinghealthisdifferentfrommaxhealth) (`StartingHealth_2_75BE2C6F43470B7F6617D4ACB4C1053B` _startinghealth)) (break `/Game/_Game/Health_And_Damage/S_StartingHealth` _returnvalue_2))
          (bind _output_get_2 (set `self.MaxHealth` _startingmaxhealth))
          (set `self.CurrentHealth` (`KismetMathLibrary.SelectFloat` _startinghealth _output_get_2 _startinghealthisdifferentfrommaxhealth)))
        (:`RowNotFound`
          (`KismetSystemLibrary.PrintText` (`|FormatText` "{OwnerName} Was Unable To Init StartingHealth, Check if the owner has Identifier and it's present in DT_StartingHealth \nFound Identifier{ID} " (`KismetSystemLibrary.GetDisplayName` (`self.GetOwner`)) (`local.ChosenTag`)) true true (struct :`R` 1.0 :`A` 1.0) 99.0))))))

(fn `StartDying`
  (`AnubisAbilitySystemLibrary.AddStatusTags` (`self.GetOwner`) (struct :`GameplayTags` (struct :`(TagName` "Status.HealthComponent.IsDying"))))
  (`self.StartDyingEvent`))