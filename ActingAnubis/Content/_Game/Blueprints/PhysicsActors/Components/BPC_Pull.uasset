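; Gravity-gun style component that pulls physics actors to a point in front of the camera and shoots them away.
; Pull input sphere-traces, then checks storage, three-point visibility and range (separate for projectiles) before grabbing via a found or created PhysicsHandle, updated on Tick.
; While held, pawn collision responses are cached and ignored.
; Shoot input restores them, releases and applies a camera-forward impulse; both actions send gameplay events to the object.
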(event `self.ReceiveBeginPlay`
  (set `self.PhysicsHandleComponent` (`self.GetPhysicsHandleComponent`)))

(event `self.ReceiveTick`
  (params (DeltaSeconds :type "Float (single-precision)"))
  (`/Engine/EditorBlueprintResources/StandardMacros.IsValid` (`PhysicsHandleComponent.GetGrabbedComponent` (`self.GetPhysicsHandleComponent`))
    (:`Is Valid`
      (`PhysicsHandleComponent.SetTargetLocationAndRotation` :`self` (`self.GetPhysicsHandleComponent`) :`NewLocation` (`.CameraLocationWithForwardScaled` (`/Game/_Game/Blueprints/Library/BP_GameplayUtilityLibrary.GetCameraTransformInfo` null 200.0))))))

(event `PullRaycast`
  (bind _pulledobject (`self.PulledObject`))
  (bind (_cameralocation _cameraforwardvector _camerarotation _cameralocationwithforwardscaled) (`/Game/_Game/Blueprints/Library/BP_GameplayUtilityLibrary.GetCameraTransformInfo` null (`KismetMathLibrary.FMax` (`self.PullRange`) (`self.ProjectilePullRange`))))
  (`/Engine/EditorBlueprintResources/StandardMacros.IsValid` (`PhysicsHandleComponent.GetGrabbedComponent` (`self.GetPhysicsHandleComponent`))
    (:`Is Not Valid`
      (if (< (`self.CurrentStorage`) (`self.MaxStorage`))
        (set `self.PulledObject` null)
        (bind _outhit (`KismetSystemLibrary.SphereTraceSingle` _cameralocation _cameralocationwithforwardscaled 100.0 "TraceTypeQuery4" false (`|MakeArray` (`self.GetOwner`)) (`self.Draw Debug Type`)))
        (bind (_bblockinghit _binitialoverlap _time _distance _location _impactpoint _normal _impactnormal _physmat _hitactor _hitcomponent) (`GameplayStatics.BreakHitResult` _outhit))
        (bind _output_get (set `self.PulledObject` _hitactor))
        (`/Engine/EditorBlueprintResources/StandardMacros.IsValid` _output_get
          (:`Is Valid`
            (bind _returnvalue (`self.PulledActorIsVisible`))
            (if _returnvalue
              (bind _returnvalue_2 (`self.CanBePulled`))
              (if _returnvalue_2
                ;[0.15 0.15 0.15 0.5 12] Same As CurrentStorage == CurrentStorage + 1
                (`/Engine/EditorBlueprintResources/StandardMacros.IncrementInt` (`self.CurrentStorage`)
                  (:`  `
                    (`self.ToggleCollisionResponseToPawns` _hitcomponent)
                    (`self.SendGameplayEvent` (struct :`TagName` "Gameplay.Event.Pull.Executed"))
                    (`PhysicsHandleComponent.GrabComponentAtLocationWithRotation` (`self.GetPhysicsHandleComponent`) _hitcomponent "None" (`Actor.K2_GetActorLocation` _pulledobject) (`Actor.K2_GetActorRotation` _pulledobject))))))))))))

(event `ListenToInputTagInterface.ReceiveTriggeredInputFromTag`
  (params (EventData :type "GameplayTag Structure"))
  (`|SwitchGameplayTag` EventData
    (:`Input.Pull.Tap`
      (`self.PullRaycast`))
    (:`Input.Shoot`
      (`self.Push`))))

(event `Push`
  (if (and (> (`self.CurrentStorage`) 0) (`KismetSystemLibrary.IsValid` (`self.PulledObject`)))
    (`/Engine/EditorBlueprintResources/StandardMacros.DecrementInt` (`self.CurrentStorage`)
      (:`  `
        (`self.ShootAndRelease`)
        (`self.ExecuteShoot`)
        (set `self.PulledObject` null)))))

(fn `CanBePulled`
  (returns (ReturnValue :type Boolean))
  (bind _returnvalue (`AnubisAbilitySystemLibrary.HasMatchingGameplayTag` (`self.PulledObject`) (struct :`TagName` "Identifier.Projectile")))
  (if _returnvalue
    (return (`/Game/_Game/Blueprints/Library/BP_MathLibrary.DistanceBetweenActorsWithinTolerance` (`self.GetOwner`) (`self.PulledObject`) (`self.ProjectilePullRange`)))
    (else
      (`AnubisAbilitySystemLibrary.HasMatchingGameplayTag` (`self.PulledObject`) (struct :`TagName` "Status.Physics.CanBePulled"))
      (return (`/Game/_Game/Blueprints/Library/BP_MathLibrary.DistanceBetweenActorsWithinTolerance` (`self.GetOwner`) (`self.PulledObject`) (`self.PullRange`))))))

(fn `ExecuteShoot`
  (`AbilitySystemBlueprintLibrary.SendGameplayEventToActor` (`self.PulledObject`) (struct :`TagName` "Gameplay.Event.Pull.Shoot") (make `GameplayEventData` :`Instigator` (`GameplayStatics.GetPlayerCharacter` 0) :`Target` (`self.PulledObject`))))

(fn `GetPhysicsHandleComponent`
  (returns (ReturnValue :type "PhysicsHandleComponent Object Reference"))
  (locals (OutPhysicsHandle :type "PhysicsHandleComponent Object Reference"))
  (`|ExecutionSequence`
    (:`then_0`
      (`self.PhysicsHandleComponent`
        (:`then`
          (return (`self.PhysicsHandleComponent`)))
        (:`else`
          (bind _output_get (set `local.OutPhysicsHandle` (`Actor.GetComponentByClass` (`self.GetOwner`) "/Script/Engine.PhysicsHandleComponent")))
          (`/Engine/EditorBlueprintResources/StandardMacros.IsValid` _output_get
            (:`Is Not Valid`
              (bind _returnvalue (`|AddComponentByClass` (`self.GetOwner`) "/Script/Engine.PhysicsHandleComponent"))
              (set `local.OutPhysicsHandle` _returnvalue))))))
    (:`then_1`
      (return (`local.OutPhysicsHandle`)))))

(fn `PulledActorIsVisible`
  (returns (ReturnValue :type Boolean))
  (locals (IgnoreActors :type "Array of Actor Object Reference") (CameraLocation :type "Vector Structure" :default (0.0 0.0 0.0)) (PulledActorLocation :type "Vector Structure" :default (0.0 0.0 0.0)) (ZBounds :type "Float (double-precision)" :default 0.0))
  (bind _pulledobject (`self.PulledObject`))
  (bind (_origin _boxextent) (`Actor.GetActorBounds` _pulledobject false false))
  (set `local.IgnoreActors` (`|MakeArray` (`self.GetOwner`) _pulledobject))
  (set `local.CameraLocation` (`/Game/_Game/Blueprints/Library/BP_GameplayUtilityLibrary.GetCameraLocation` null))
  (set `local.PulledActorLocation` _origin)
  (set `local.ZBounds` (- (.z _boxextent) (`self.ZBoundsOffset`)))
  (`|ExecutionSequence`
    (:`then_0`
      (bind (_outhit _returnvalue) (`KismetSystemLibrary.LineTraceSingle` (`local.CameraLocation`) (`local.PulledActorLocation`) "TraceTypeQuery1" false (`local.IgnoreActors`) (`self.Draw Debug Type`)))
      (if (not _returnvalue)
        (return true)))
    (:`then_1`
      (bind (_outhit_2 _returnvalue_2) (`KismetSystemLibrary.LineTraceSingle` (`local.CameraLocation`) (+ (`local.PulledActorLocation`) (`KismetMathLibrary.MakeVector` 0.0 0.0 (`local.ZBounds`))) "TraceTypeQuery1" false (`local.IgnoreActors`) (`self.Draw Debug Type`)))
      (if (not _returnvalue_2)
        (return true)))
    (:`then_2`
      (bind (_outhit_3 _returnvalue_3) (`KismetSystemLibrary.LineTraceSingle` (`local.CameraLocation`) (- (`local.PulledActorLocation`) (`KismetMathLibrary.MakeVector` 0.0 0.0 (`local.ZBounds`))) "TraceTypeQuery1" false (`local.IgnoreActors`) (`self.Draw Debug Type`)))
      (if (not _returnvalue_3)
        (return true)))
    (:`then_3`
      (return false))))

(fn `RelativeTransform`
  (returns (ReturnValue :type "Transform Structure"))
  (return))

(fn `SendGameplayEvent`
  (params (EventTag :type "GameplayTag Structure"))
  (bind _pulledobject (`self.PulledObject`)
    (:`then`
      (`AbilitySystemBlueprintLibrary.SendGameplayEventToActor` _pulledobject EventTag (make `GameplayEventData` :`Instigator` (`self.GetOwner`) :`Target` (`self.PulledObject`))))
    (:`else`)))

(fn `ShootAndRelease`
  (locals (PrimitiveComponent :type "PrimitiveComponent Object Reference"))
  (bind _physicshandlecomponent (`self.PhysicsHandleComponent`))
  (bind _returnvalue (`PhysicsHandleComponent.GetGrabbedComponent` _physicshandlecomponent))
  (bind _output_get (set `local.PrimitiveComponent` _returnvalue))
  (`self.ToggleCollisionResponseToPawns` _returnvalue true)
  (`PhysicsHandleComponent.ReleaseComponent` _physicshandlecomponent)
  (`/Game/_Game/Blueprints/Library/BP_GameplayLibrary.ExecutePushOnPushableObject` (`self.PulledObject`) _output_get (`self.GetOwner`) (`/Game/_Game/Blueprints/Library/BP_GameplayUtilityLibrary.GetCameraForwardVector` null) (`self.ShootingSpeed`)))

(fn `StoreWaitAsyncTask`
  (params (WaitGameplayEvent :type "AbilityAsync_WaitGameplayEvent Object Reference"))
  (returns (ReturnValue :type Boolean))
  (return false))

(fn `ToggleCollisionResponseToPawns`
  (params (PrimComp :type "PrimitiveComponent Object Reference") (TurnOn :type Boolean))
  (bind _cachedresponses (`self.CachedResponses`))
  (bind _primcomp (`local.PrimComp`))
  (if TurnOn
    (bind _keys (`BlueprintMapLibrary.Map_Keys` _cachedresponses))
    (for _array_element _keys
      (`PrimitiveComponent.SetCollisionResponseToChannel` (`local.PrimComp`) _array_element (`BlueprintMapLibrary.Map_Find` _cachedresponses _array_element)))
    (else
      (`BlueprintMapLibrary.Map_Add` _cachedresponses "ECC_GameTraceChannel5" (`PrimitiveComponent.GetCollisionResponseToChannel` _primcomp "ECC_GameTraceChannel5"))
      (`BlueprintMapLibrary.Map_Add` _cachedresponses "ECC_Pawn" (`PrimitiveComponent.GetCollisionResponseToChannel` _primcomp "ECC_Pawn"))
      (bind _keys_2 (`BlueprintMapLibrary.Map_Keys` _cachedresponses))
      (for _array_element_2 _keys_2
        (`PrimitiveComponent.SetCollisionResponseToChannel` (`local.PrimComp`) _array_element_2 "ECR_Ignore")))))