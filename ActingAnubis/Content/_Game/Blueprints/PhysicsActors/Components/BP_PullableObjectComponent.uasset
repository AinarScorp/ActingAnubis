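; Actor component that lets its owner be pulled in and stored by the first-person character, then shot back out.
; It listens for gameplay events on the owner: Pull Executed disables physics and attaches the owner to the character's Storage component.
; Pull Shoot detaches it, teleports it to the ShootPoint, re-enables physics and applies a velocity-change impulse along the camera's forward vector.
; Physics changes require a primitive root component; resize logic exists but is unconnected.
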(event `self.ReceiveBeginPlay`
  (bind _returnvalue (`self.GetOwner`))
  (bind _returnvalue_2 (`self.GetOwner`))
  (`|ExecutionSequence`
    (:`then_0`
      (`AbilityAsync_WaitGameplayEvent.WaitGameplayEventToActor` _returnvalue_2 (struct :`TagName` "Gameplay.Event.Pull.Executed")
        (:`EventReceived`
          (`self.SetSimulatingPhysics` false)
          (bind _asbp_first_person_character (cast `/Game/_Game/Blueprints/Player/BP_FirstPersonCharacter` (`GameplayStatics.GetPlayerCharacter` 0)))
          (`Actor.K2_AttachToComponent` _returnvalue_2 (`/Game/_Game/Blueprints/Player/BP_FirstPersonCharacter.Storage` _asbp_first_person_character) "None" "SnapToTarget" "SnapToTarget" "KeepRelative" false))))
    (:`then_1`
      (`AbilityAsync_WaitGameplayEvent.WaitGameplayEventToActor` _returnvalue (struct :`TagName` "Gameplay.Event.Pull.Shoot")
        (:`EventReceived`
          (bind _asbp_first_person_character_2 (cast `/Game/_Game/Blueprints/Player/BP_FirstPersonCharacter` (`GameplayStatics.GetPlayerCharacter` 0)))
          (`Actor.K2_DetachFromActor` _returnvalue "KeepWorld" "KeepWorld" "KeepWorld")
          (`Actor.K2_SetActorLocation` _returnvalue (`SceneComponent.K2_GetComponentLocation` (`/Game/_Game/Blueprints/Player/BP_FirstPersonCharacter.ShootPoint` _asbp_first_person_character_2)) false true)
          (bind (_bsuccess _asprimitive_component) (`self.GetPrimitiveComponent`))
          (if _bsuccess
            (`self.SetSimulatingPhysics` true)
            (`PrimitiveComponent.AddImpulse` _asprimitive_component (* (`SceneComponent.GetForwardVector` (`/Game/_Game/Blueprints/Player/BP_FirstPersonCharacter.FirstPersonCamera` _asbp_first_person_character_2)) (`self.ShootingSpeed`)) "None" true)))))))

(fn `GetPrimitiveComponent`
  (returns (bSuccess :type Boolean) (`AsPrimitive Component` :type "PrimitiveComponent Object Reference"))
  (bind _asprimitive_component (cast `PrimitiveComponent` (`Actor.RootComponent` (`self.GetOwner`)))
    (:`then`
      (return true _asprimitive_component))
    (:`CastFailed`
      (return false null))))

(fn `SetSimulatingPhysics`
  (params (NewSimulate :type Boolean))
  (bind (_bsuccess _asprimitive_component) (`self.GetPrimitiveComponent`))
  (if _bsuccess
    (`PrimitiveComponent.SetSimulatePhysics` _asprimitive_component NewSimulate)))