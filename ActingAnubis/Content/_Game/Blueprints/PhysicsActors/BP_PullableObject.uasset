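; BP_PullableObject is a physics prop that damages enemies it hits after being shot by the pull mechanic.
; A Gameplay.Event.Pull.Shoot event enables hit notifications, and the first hit disables them, applying fixed damage credited to the player if the target is an enemy.
; RandomizeAndSetMesh picks a mesh and random scale from per-mesh info, with index and mesh overrides.
; The collision box sizing logic is disconnected, so SetCollisionBoxSize currently does nothing.
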(event `self.ReceiveBeginPlay`
  (`AbilityAsync_WaitGameplayEvent.WaitGameplayEventToActor` null (struct :`TagName` "Gameplay.Event.Pull.Shoot")
    (:`EventReceived`
      (`PrimitiveComponent.SetNotifyRigidBodyCollision` (`self.StaticMesh`) true))))

(event `SetCollisionBox Size`
  (`self.SetCollisionBox`))

(event `RandomizeAndSetMesh`
  (bind _staticmesh (`self.StaticMesh`))
  (bind (_mesh _scalemin _scalemax) (break `/Game/_Game/Blueprints/PhysicsActors/Structs/S_MeshInfos` (`self.GetCurrentMeshInfo`)))
  (`self.SetNewRandomIndex`)
  (`StaticMeshComponent.SetStaticMesh` _staticmesh _mesh)
  (`SceneComponent.SetWorldScale3D` _staticmesh (`KismetMathLibrary.MakeVector` (`KismetMathLibrary.RandomFloatInRange` (.x _scalemin) (.x _scalemax)) (`KismetMathLibrary.RandomFloatInRange` (.y _scalemin) (.y _scalemax)) (`KismetMathLibrary.RandomFloatInRange` (.z _scalemin) (.z _scalemax)))))

(event `self.StaticMesh.OnComponentHit`
  (params (HitComponent :type "PrimitiveComponent Object Reference") (OtherActor :type "Actor Object Reference") (OtherComp :type "PrimitiveComponent Object Reference") (NormalImpulse :type "Vector Structure") (Hit :type "HitResult Structure (by ref)"))
  (`|ExecutionSequence`
    (:`then_0`
      (bind _returnvalue (`AnubisAbilitySystemLibrary.HasMatchingGameplayTag` OtherActor (struct :`TagName` "Identifier.Enemy")))
      (if _returnvalue
        (`/Game/_Game/Blueprints/Library/BP_GameplayLibrary.DealDamageToActor` OtherActor (`GameplayStatics.GetPlayerCharacter` 0) 50.0)))
    (:`then_1`
      (`PrimitiveComponent.SetNotifyRigidBodyCollision` (`self.StaticMesh`) false))))

(fn `GetCurrentMeshInfo`
  (returns (ReturnValue :type "/Game/_Game/Blueprints/PhysicsActors/Structs/S_MeshInfos Structure"))
  (bind _overrideindex (`self.OverrideIndex`))
  (bind _output_get (set `self.CurrentIndex(DebugOnly)` (`KismetMathLibrary.SelectInt` (`self.RandomMeshIndex`) _overrideindex (< _overrideindex 0))))
  (return (select `bool` (`self.bShouldOverrideMesh`) :`false` (`|GetArrayItem` (`self.Meshes`) _output_get) :`true` (`self.bOverrideMesh`))))

(fn `SetCollisionBox`
  (locals (CachedWorldScale :type "Vector Structure" :default (0.0 0.0 0.0)) (ActorRotCached :type "Rotator Structure" :default (struct))))

(fn `SetNewRandomIndex`
  (if (< (`self.OverrideIndex`) 0)
    (set `self.RandomMeshIndex` (`KismetMathLibrary.RandomIntegerInRange` 0 (`KismetArrayLibrary.Array_LastIndex` (`self.Meshes`))))))

(fn `UserConstructionScript`)