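; Explosive barrel physics actor with a tintable material that detonates after being launched by a physics impulse.
; An Impulse gameplay event saves the instigator and enables hit and overlap events for ten seconds.
; A hard hit or pawn overlap spawns an explosion, sphere-traces the radius with debug drawing, then destroys the barrel.
; Each traced actor is processed once: destructible walls are destroyed, others take damage and an outward push credited to the instigator.
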(event `self.ReceiveBeginPlay`
  ; If you wanna use me, Add Anubis SIMPLE AbilitySystem
  (bind (_asynctaskproxy _payload) (`AbilityAsync_WaitGameplayEvent.WaitGameplayEventToActor` null (struct :`TagName` "Gameplay.Event.Physics.Impulse"))
    (:`EventReceived`
      (`self.SaveInsitgator` _payload)
      (set `PrimitiveComponent.bGenerateOverlapEvents` true (`self.StaticMesh`))
      (`PrimitiveComponent.SetNotifyRigidBodyCollision` (`self.StaticMesh`) true)
      (`KismetSystemLibrary.Delay` 10.0)
      (`PrimitiveComponent.SetNotifyRigidBodyCollision` (`self.StaticMesh`) false)
      (set `PrimitiveComponent.bGenerateOverlapEvents` false (`self.StaticMesh`)))))

(event `self.ReceiveTick`
  (params (DeltaSeconds :type "Float (single-precision)")))

(event `self.StaticMesh.OnComponentHit`
  (params (HitComponent :type "PrimitiveComponent Object Reference") (OtherActor :type "Actor Object Reference") (OtherComp :type "PrimitiveComponent Object Reference") (NormalImpulse :type "Vector Structure") (Hit :type "HitResult Structure (by ref)"))
  (bind _returnvalue (`self.K2_GetActorLocation`))
  (if (> (`KismetMathLibrary.VSize` NormalImpulse) 10000.0)
    (`self.HandlePhysics` :!label _label)
    (`GameplayStatics.SpawnEmitterAtLocation` "/Game/StarterContent/Particles/P_Explosion.P_Explosion" (`self.K2_GetActorLocation`) (struct) (3.0 3.0 3.0))
    (bind _outhits (`KismetSystemLibrary.SphereTraceMulti` :`Start` _returnvalue :`End` _returnvalue :`Radius` (`self.ExplodeRadius`) :`TraceChannel` "TraceTypeQuery3" :`DrawDebugType` "ForDuration"))
    (`self.HandleHits` _outhits)
    (`self.K2_DestroyActor`)))

(event `self.StaticMesh.OnComponentBeginOverlap`
  (params (OverlappedComponent :type "PrimitiveComponent Object Reference") (OtherActor :type "Actor Object Reference") (OtherComp :type "PrimitiveComponent Object Reference") (OtherBodyIndex :type Integer) (bFromSweep :type Boolean) (SweepResult :type "HitResult Structure (by ref)"))
  (cast `Pawn` OtherActor)
  (`KismetSystemLibrary.PrintString` (`KismetSystemLibrary.GetDisplayName` OtherComp))
  (goto _label))

(fn `HandleHits`
  (params (Array :type "Array of HitResult Structure"))
  (locals (ProcessedActors :type "Array of Actor Object Reference") (HitActor :type "Actor Object Reference"))
  (bind _impulseinsigator (`self.ImpulseInsigator`))
  (bind _hitactor (`local.HitActor`))
  (for _array_element Array
    (bind (_bblockinghit _binitialoverlap _time _distance _location _impactpoint _normal _impactnormal _physmat _hitactor_2 _hitcomponent) (`GameplayStatics.BreakHitResult` _array_element))
    (bind _output_get (set `local.HitActor` _hitactor_2))
    (if (not (`KismetArrayLibrary.Array_Contains` (`local.ProcessedActors`) _output_get))
      (`KismetArrayLibrary.Array_Add` (`local.ProcessedActors`) _hitactor)
      (bind _returnvalue (`AnubisAbilitySystemLibrary.HasMatchingGameplayTag` _hitactor (struct :`TagName` "Identifier.DestructableWall")))
      (if _returnvalue
        (`self.K2_DestroyActor` _hitactor)
        (else
          (`/Game/_Game/Blueprints/Library/BP_GameplayLibrary.DealDamageToActor` _hitactor _impulseinsigator 50.0)
          (`/Game/_Game/Blueprints/Library/BP_GameplayLibrary.ExecutePushOnPushableObject` _hitactor _hitcomponent _impulseinsigator (`KismetMathLibrary.GetDirectionUnitVector` (`self.K2_GetActorLocation`) (`self.K2_GetActorLocation` (`local.HitActor`))) 2000.0))))))

(fn `HandlePhysics`
  (bind _staticmesh (`self.StaticMesh`))
  (`PrimitiveComponent.SetSimulatePhysics` _staticmesh false)
  (`PrimitiveComponent.SetCollisionEnabled` _staticmesh "NoCollision"))

(fn `SaveInsitgator`
  (params (GameplayEventData :type "GameplayEventData Structure (by ref)"))
  (bind (_eventtag _instigator) (break `GameplayEventData` GameplayEventData))
  (set `self.ImpulseInsigator` (select `bool` (`KismetSystemLibrary.IsValid` _instigator) :`false` self :`true` _instigator :!type "Actor Object Reference")))

(fn `UserConstructionScript`
  (bind _returnvalue (`PrimitiveComponent.CreateDynamicMaterialInstance` (`self.StaticMesh`) 0 "/Engine/BasicShapes/BasicShapeMaterial_Inst.BasicShapeMaterial_Inst" "None"))
  (`MaterialInstanceDynamic.SetScalarParameterValue` _returnvalue "Roughness" 1.0)
  (`MaterialInstanceDynamic.SetVectorParameterValue` _returnvalue "Color" (`self.MaterialColor`)))