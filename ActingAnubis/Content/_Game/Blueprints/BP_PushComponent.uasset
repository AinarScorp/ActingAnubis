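; Actor component that gives its owner a push, launching objects away from it along the player's view.
; ExecutePush box-traces ahead of the owner using player 0's controller forward vector and control rotation, with debug drawing.
; Each hit actor gets a sphere-trace visibility check, and unblocked ones receive a velocity-change impulse away from the owner.
; Tagged input events only print their tag, and a helper stores a gameplay-event wait task.
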(event `self.ReceiveBeginPlay`
  (`KismetSystemLibrary.PrintString` "CREATED"))

(event `ExecutePush`
  (bind (_starttracelocation _endtracelocation _orientation) (`self.GetTraceParams`))
  (bind _outhits (`KismetSystemLibrary.BoxTraceMulti` :`Start` _starttracelocation :`End` _endtracelocation :`HalfSize` (`self.Half Size`) :`Orientation` _orientation :`TraceChannel` "TraceTypeQuery3" :`DrawDebugType` "ForDuration"))
  (for _array_element _outhits
    (bind (_bblockinghit _binitialoverlap _time _distance _location _impactpoint _normal _impactnormal _physmat _hitactor _hitcomponent) (`GameplayStatics.BreakHitResult` _array_element))
    (`/Engine/EditorBlueprintResources/StandardMacros.IsValid` _hitactor
      (:`Is Valid`
        (bind _returnvalue (`Actor.K2_GetActorLocation` _hitactor))
        (bind (_outhit _returnvalue_2) (`KismetSystemLibrary.SphereTraceSingle` :`Start` (`Actor.K2_GetActorLocation` (`self.GetOwner`)) :`End` _returnvalue :`Radius` 25.0 :`TraceChannel` "TraceTypeQuery1" :`DrawDebugType` "ForDuration"))
        (if (not _returnvalue_2)
          (`PrimitiveComponent.AddImpulse` _hitcomponent (* (`KismetMathLibrary.GetDirectionUnitVector` (`Actor.K2_GetActorLocation` (`self.GetOwner`)) _returnvalue) 3000.0) "None" true))))))

(event `ListenToInputTagInterface.ReceiveTriggeredInputFromTag`
  (params (EventData :type "GameplayTag Structure"))
  (`KismetSystemLibrary.PrintString` (`KismetStringLibrary.Conv_NameToString` (`BlueprintGameplayTagLibrary.GetTagName` EventData))))

(event `ListenToInputTagInterface.ReceiveReleasedInputFromTag`
  (params (EventData :type "GameplayTag Structure"))
  (`KismetSystemLibrary.PrintString` (`KismetStringLibrary.Conv_NameToString` (`BlueprintGameplayTagLibrary.GetTagName` EventData))))

(fn `GetTraceParams`
  (returns (StartTraceLocation :type "Vector Structure") (EndTraceLocation :type "Vector Structure") (Orientation :type "Rotator Structure"))
  (bind _returnvalue (`GameplayStatics.GetPlayerController` 0))
  (bind _half_size_x (`KismetMathLibrary.BreakVector` (`self.Half Size`)))
  (bind _returnvalue_2 (`Actor.GetActorForwardVector` _returnvalue))
  (bind _returnvalue_3 (+ (`Actor.K2_GetActorLocation` (`self.GetOwner`)) (* _returnvalue_2 _half_size_x)))
  (return _returnvalue_3 (+ _returnvalue_3 (* _returnvalue_2 (`self.TraceLength`))) (`Controller.GetControlRotation` _returnvalue)))

(fn `RelativeTransform`
  (returns (ReturnValue :type "Transform Structure"))
  (return (`KismetMathLibrary.MakeTransform` (1.0 2.0 3.0) (struct :`Pitch` 4.0 :`Yaw` 5.0 :`Roll` 40.0) (6.0 7.0 8.0))))

(fn `StoreWaitAsyncTask`
  (params (WaitGameplayEvent :type "AbilityAsync_WaitGameplayEvent Object Reference"))
  (returns (ReturnValue :type Boolean))
  (set `self.Wait Gameplay Event` WaitGameplayEvent)
  (return true))

(fn `WORK`
  (returns (ReturnValue :type "ListenToInputTagInterface Interface"))
  (return self))